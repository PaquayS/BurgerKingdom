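; AI character that spawns with a randomized accessory look, walks a fixed four-waypoint route and destroys itself at the end.
; BeginPlay hides its Plane, finds BP_WaypointSystem1 and chains AIMoveTo calls with short delays, handling only success.
; The construction script picks skeletal meshes through nested 1-in-18 rolls, favoring earlier variants and sometimes keeping the default.
; AttachPlate forwards attachment to the plate; GradeHappiness is an empty stub.
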(event `InitiateActor`
  (bind _returnvalue (`GameplayStatics.GetActorOfClass` "/Game/Cproef/Blueprints/AI/BP_WaypointSystem1.BP_WaypointSystem1_C"))
  (set `self.WP` _returnvalue)
  (`self.Walking`))

(event `self.ReceiveBeginPlay`
  (`self.InitiateActor`)
  (`SceneComponent.SetVisibility` (`self.Plane`) false false))

(event `Walking`
  (`|AIMoveTo` self (0.0 0.0 0.0) (`/Game/Cproef/Blueprints/AI/BP_WaypointSystem1.Waypoint1` (`self.WP`))
    (:`OnSuccess`
      (`KismetSystemLibrary.Delay` 0.2)
      (`|AIMoveTo` self (0.0 0.0 0.0) (`/Game/Cproef/Blueprints/AI/BP_WaypointSystem1.Waypoint2` (`self.WP`))
        (:`OnSuccess`
          (`KismetSystemLibrary.Delay` 0.2)
          (`|AIMoveTo` self (0.0 0.0 0.0) (`/Game/Cproef/Blueprints/AI/BP_WaypointSystem1.Waypoint3` (`self.WP`))
            (:`OnSuccess`
              (`KismetSystemLibrary.Delay` 0.2)
              (`|AIMoveTo` self (0.0 0.0 0.0) (`/Game/Cproef/Blueprints/AI/BP_WaypointSystem1.Waypoint4` (`self.WP`))
                (:`OnSuccess`
                  (`KismetSystemLibrary.Delay` 0.2)
                  (`self.K2_DestroyActor`))))))))))

(fn `AttachPlate`
  (params (AttachParent :type "SceneComponent Object Reference") (Plate :type "/Game/Cproef/Blueprints/Cooking/BP_Plate Object Reference"))
  (`/Game/Cproef/Blueprints/Cooking/BP_Plate.AttachToAI` Plate AttachParent))

(fn `GradeHappiness`)

(fn `UserConstructionScript`
  (bind _returnvalue (`KismetMathLibrary.RandomInteger` 18))
  (bind _mesh (`self.Mesh`))
  (bind _mesh_2 (`self.Mesh`))
  (bind _mesh_3 (`self.Mesh`))
  (bind _mesh_4 (`self.Mesh`))
  (bind _mesh_5 (`self.Mesh`))
  (bind _mesh_6 (`self.Mesh`))
  (if (== _returnvalue 0)
    (`SkinnedMeshComponent.SetSkinnedAssetAndUpdate` _mesh_3 "/Game/Cproef/Models/AI/AI1/AI_Glasses.AI_Glasses" true)
    (elif (== _returnvalue 0)
      (`SkinnedMeshComponent.SetSkinnedAssetAndUpdate` _mesh_3 "/Game/Cproef/Models/AI/AI2/AI_Glasses_Hat.AI_Glasses_Hat" true)
      (elif (== _returnvalue 0)
        (`SkinnedMeshComponent.SetSkinnedAssetAndUpdate` _mesh_3 "/Game/Cproef/Models/AI/AI3/AI_Glasses_Mohawk.AI_Glasses_Mohawk" true)
        (elif (== _returnvalue 0)
          (`SkinnedMeshComponent.SetSkinnedAssetAndUpdate` _mesh_4 "/Game/Cproef/Models/AI/AI4/AI_Glasses_PoliceHat.AI_Glasses_PoliceHat" true)
          (elif (== _returnvalue 0)
            (`SkinnedMeshComponent.SetSkinnedAssetAndUpdate` _mesh_4 "/Game/Cproef/Models/AI/AI5/AI_Glasses_Sunhat.AI_Glasses_Sunhat" true)
            (elif (== _returnvalue 0)
              (`SkinnedMeshComponent.SetSkinnedAssetAndUpdate` _mesh_4 "/Game/Cproef/Models/AI/AI6/AI_Glasses_Tophat.AI_Glasses_Tophat" true)
              (elif (== _returnvalue 0)
                (`SkinnedMeshComponent.SetSkinnedAssetAndUpdate` _mesh_5 "/Game/Cproef/Models/AI/AI_Monocle/AI1/AI_Monocle.AI_Monocle" true)
                (elif (== _returnvalue 0)
                  (`SkinnedMeshComponent.SetSkinnedAssetAndUpdate` _mesh_5 "/Game/Cproef/Models/AI/AI_Monocle/AI2/AI_Monocle_Hat.AI_Monocle_Hat" true)
                  (elif (== _returnvalue 0)
                    (`SkinnedMeshComponent.SetSkinnedAssetAndUpdate` _mesh_5 "/Game/Cproef/Models/AI/AI_Monocle/AI_Monocle_Mohawk.AI_Monocle_Mohawk" true)
                    (elif (== _returnvalue 0)
                      (`SkinnedMeshComponent.SetSkinnedAssetAndUpdate` _mesh_6 "/Game/Cproef/Models/AI/AI_Monocle/AI_Monocle_PoliceHat.AI_Monocle_PoliceHat" true)
                      (elif (== _returnvalue 0)
                        (`SkinnedMeshComponent.SetSkinnedAssetAndUpdate` _mesh_6 "/Game/Cproef/Models/AI/AI_Monocle/AI_Monocle_SunHat.AI_Monocle_SunHat" true)
                        (elif (== _returnvalue 0)
                          (`SkinnedMeshComponent.SetSkinnedAssetAndUpdate` _mesh_6 "/Game/Cproef/Models/AI/AI_Monocle/AI_Monocle_TopHat.AI_Monocle_TopHat" true)
                          (elif (== _returnvalue 0)
                            (`SkinnedMeshComponent.SetSkinnedAssetAndUpdate` _mesh_2 "/Game/Cproef/Models/AI/AI_SunGlasses/AI1/AI_Sunglasses.AI_Sunglasses" true)
                            (elif (== _returnvalue 0)
                              (`SkinnedMeshComponent.SetSkinnedAssetAndUpdate` _mesh_2 "/Game/Cproef/Models/AI/AI_SunGlasses/AI2/AI_Sunglasses_Hat.AI_Sunglasses_Hat" true)
                              (elif (== _returnvalue 0)
                                (`SkinnedMeshComponent.SetSkinnedAssetAndUpdate` _mesh_2 "/Game/Cproef/Models/AI/AI_SunGlasses/AI3/AI_Sunglasses_Mohawk.AI_Sunglasses_Mohawk" true)
                                (elif (== _returnvalue 0)
                                  (`SkinnedMeshComponent.SetSkinnedAssetAndUpdate` _mesh "/Game/Cproef/Models/AI/AI_SunGlasses/AI4/AI_SunGlasses_PoliceHat.AI_SunGlasses_PoliceHat" true)
                                  (elif (== _returnvalue 0)
                                    (`SkinnedMeshComponent.SetSkinnedAssetAndUpdate` _mesh "/Game/Cproef/Models/AI/AI_SunGlasses/AI5/AI_Sunglasses_SunHat.AI_Sunglasses_SunHat" true)
                                    (elif (== _returnvalue 0)
                                      (`SkinnedMeshComponent.SetSkinnedAssetAndUpdate` _mesh "/Game/Cproef/Models/AI/AI_SunGlasses/AI6/AI_SunGlasses_TopHat.AI_SunGlasses_TopHat" true))))))))))))))))))))