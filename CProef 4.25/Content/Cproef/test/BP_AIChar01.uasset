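; Restaurant customer AI that queues along BP_WaypointSystem waypoints, orders a random burger or pizza shown on a plane, and leaves after pickup.
; Queue spots are polled with delays; waiting too long, or food-related actors overlapping CheckFood, makes it leave angry.
; FoodPickUp scores the order against BP_AIOrder to grade mood, plays sounds and attaches the plate.
; The construction script randomizes the head-accessory mesh through chained random rolls.
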(event `self.ReceiveTick`
  (params (DeltaSeconds :type "Float (single-precision)"))
  (bind _returnvalue (`GameplayStatics.GetActorOfClass` "/Game/Cproef/Blueprints/AI/BP_AIOrder.BP_AIOrder_C"))
  (set `self.Order` _returnvalue))

(event `InitiateActor`
  (bind _returnvalue (`GameplayStatics.GetActorOfClass` "/Game/Cproef/Blueprints/AI/BP_WaypointSystem.BP_WaypointSystem_C"))
  (set `self.Waypoints` _returnvalue)
  (`self.WaitingLine`))

(event `self.ReceiveBeginPlay`
  (`self.InitiateActor`)
  (`SceneComponent.SetVisibility` (`self.Plane`) false false))

(event `WaitingLine`
  (bind _waypoints (`self.Waypoints`))
  (bind _waypoints_2 (`self.Waypoints`))
  (if (`/Game/Cproef/Blueprints/AI/BP_WaypointSystem.Spot3Filled?` (`self.Waypoints`)) :!label _label
    (`KismetSystemLibrary.Delay` 5.0)
    (goto _label)
    (else
      ;[1 1 1] Moves AI to 3spot in waiting line
      (`|AIMoveTo` self (0.0 0.0 0.0) (`/Game/Cproef/Blueprints/AI/BP_WaypointSystem.Waypoint3` (`self.Waypoints`))
        (:`OnSuccess`
          (`KismetSystemLibrary.Delay` 0.2)
          ;[1 1 1] checks if next spot is free to move too
          (if (`/Game/Cproef/Blueprints/AI/BP_WaypointSystem.Spot2Filled?` (`self.Waypoints`)) :!label _label_2
            ;[1 1 1] checks how long the AI has been waiting without moving
            (bind _output_get (set `self.delayFrequenty?` (+ (`self.delayFrequenty?`) 1.0)))
            (if (>= _output_get 3.0)
              (set `self.Angrery?` true)
              ;[1 1 1] Makes AI leave if to long in waiting line
              (`KismetSystemLibrary.Delay` 2.5)
              (`|AIMoveTo` self (0.0 0.0 0.0) (`/Game/Cproef/Blueprints/AI/BP_WaypointSystem.Waypoint4` _waypoints)
                (:`OnSuccess`
                  (`KismetSystemLibrary.Delay` 0.05)
                  (`|AIMoveTo` self (0.0 0.0 0.0) (`/Game/Cproef/Blueprints/AI/BP_WaypointSystem.Waypoint5` _waypoints)
                    (:`OnSuccess`
                      (`KismetSystemLibrary.Delay` 0.05)
                      (`|AIMoveTo` self (0.0 0.0 0.0) (`/Game/Cproef/Blueprints/AI/BP_WaypointSystem.Waypoint6` _waypoints)
                        (:`OnSuccess`
                          (`self.K2_DestroyActor`)))))))
              (else
                (`KismetSystemLibrary.Delay` 5.0)
                (goto _label_2)))
            (else
              (`|AIMoveTo` self (0.0 0.0 0.0) (`/Game/Cproef/Blueprints/AI/BP_WaypointSystem.Waypoint2` (`self.Waypoints`))
                (:`OnSuccess`
                  (`KismetSystemLibrary.Delay` 0.2)
                  (if (`/Game/Cproef/Blueprints/AI/BP_WaypointSystem.Spot1Filled?` (`self.Waypoints`)) :!label _label_3
                    (bind _output_get_2 (set `self.delayFrequenty?` (+ (`self.delayFrequenty?`) 1.0)))
                    (if (>= _output_get_2 3.0)
                      ;[1 1 1] Makes AI leave if to long in waiting line
                      (set `self.Angrery?` true)
                      (`KismetSystemLibrary.Delay` 2.5)
                      (`|AIMoveTo` self (0.0 0.0 0.0) (`/Game/Cproef/Blueprints/AI/BP_WaypointSystem.Waypoint4` _waypoints_2)
                        (:`OnSuccess`
                          (`|AIMoveTo` self (0.0 0.0 0.0) (`/Game/Cproef/Blueprints/AI/BP_WaypointSystem.Waypoint5` _waypoints_2)
                            (:`OnSuccess`
                              (`|AIMoveTo` self (0.0 0.0 0.0) (`/Game/Cproef/Blueprints/AI/BP_WaypointSystem.Waypoint6` _waypoints_2)
                                (:`OnSuccess`
                                  (`self.K2_DestroyActor`)))))))
                      (else
                        (`KismetSystemLibrary.Delay` 5.0)
                        (goto _label_3)))
                    (else
                      (`|AIMoveTo` self (0.0 0.0 0.0) (`/Game/Cproef/Blueprints/AI/BP_WaypointSystem.Waypoint1` (`self.Waypoints`))
                        (:`OnSuccess`
                          ;[1 1 1] AI can order here
                          (set `self.canOrder?` true)
                          (`self.Ordering`)
                          (set `self.ordered?` true)
                          (`SceneComponent.SetVisibility` (`self.Plane`) true false)
                          (set `self.Idle?` true))))))))))))))

(event `Ordering`
  ;[1 1 1] generationg a random int and checking the value
  (switch `int` (`KismetMathLibrary.RandomInteger` (enumcount `/Game/Cproef/Blueprints/AI/Enum_Orders`))
    (:`Default`
      ;[1 1 1] just to fill up false, should never happen.. normally..
      (`KismetSystemLibrary.PrintString` "welp unlucky"))
    (:`0`
      ;[1 1 1] determing what to order depending on the randomly generated int
      (set `self.burger?` true)
      (`PrimitiveComponent.SetMaterial` (`self.Plane`) 0 "/Game/Cproef/Textures/M_OrderBurger.M_OrderBurger"))
    (:`1`
      (set `self.CheeseBurger` true)
      (`PrimitiveComponent.SetMaterial` (`self.Plane`) 0 "/Game/Cproef/Textures/M_OrderCheeseBurger.M_OrderCheeseBurger"))
    (:`2`
      (set `self.Pizza?` true)
      (`PrimitiveComponent.SetMaterial` (`self.Plane`) 0 "/Game/Cproef/Textures/M_OrderPizzaSalami.M_OrderPizzaSalami"))
    (:`3`
      (set `self.PizzaPaprika?` true)
      (`PrimitiveComponent.SetMaterial` (`self.Plane`) 0 "/Game/Cproef/Textures/M_OrderPizzaVeggie.M_OrderPizzaVeggie"))))

(event `FoodPickUp`
  (params (PlateToPickup :type "/Game/Cproef/Blueprints/Cooking/BP_Plate Object Reference"))
  (`self.Happiness?`)
  (`self.AudioMaker`)
  (`/Engine/EditorBlueprintResources/StandardMacros.DoOnce` false
    (:`Completed`
      (`GameplayStatics.PlaySoundAtLocation` "/Game/Cproef/Audio/Kaching.Kaching" (-110.0 -3.0 105.0) (struct) 1.0 1.0 0.0 null null null)
      (`KismetSystemLibrary.Delay` 2.0)
      (`KismetSystemLibrary.Delay` 1.0)
      (`self.AttachPlate` (`self.FoodHolder`) PlateToPickup)
      (`SceneComponent.K2_SetWorldRotation` (`Actor.RootComponent` PlateToPickup) (`KismetMathLibrary.MakeRotator` 0.0 0.0 90.0) false false)
      (`PrimitiveComponent.SetCollisionEnabled` (`StaticMeshActor.StaticMeshComponent` PlateToPickup) "NoCollision")
      (`KismetSystemLibrary.Delay` 1.0)
      (`SceneComponent.SetVisibility` (`self.Plane`) false false)
      (set `self.Idle?` false)
      (set `self.HoldingPlate?` true)
      (`|AIMoveTo` self (0.0 0.0 0.0) (`/Game/Cproef/Blueprints/AI/BP_WaypointSystem.Waypoint4` (`self.Waypoints`))
        (:`OnSuccess`
          (`|AIMoveTo` self (0.0 0.0 0.0) (`/Game/Cproef/Blueprints/AI/BP_WaypointSystem.Waypoint5` (`self.Waypoints`))
            (:`OnSuccess`
              (`|AIMoveTo` self (0.0 0.0 0.0) (`/Game/Cproef/Blueprints/AI/BP_WaypointSystem.Waypoint7` (`self.Waypoints`))
                (:`OnSuccess`
                  (`self.K2_DestroyActor`))))))))))

(event `AcceptedOrder`)

(event `AudioMaker`
  (bind _returnvalue (`KismetMathLibrary.RandomIntegerInRange` 0 2))
  (bind _audio (`self.Audio`))
  (if (`self.Angrery?`)
    (if (== _returnvalue 0)
      (`AudioComponent.SetSound` _audio "/Game/Cproef/Audio/Angry1.Angry1")
      (`AudioComponent.Play` (`self.Audio`) 0.0 :!label _label_4)
      (`KismetSystemLibrary.Delay` 0.6)
      (`AudioComponent.Stop` (`self.Audio`))
      (elif (== _returnvalue 1)
        (`AudioComponent.SetSound` _audio "/Game/Cproef/Audio/angry2.angry2")
        (goto _label_4)
        (elif (== _returnvalue 2)
          (`AudioComponent.SetSound` (`self.Audio`) "/Game/Cproef/Audio/Angry3.Angry3")
          (goto _label_4))))))

(event `Happiness?`
  (bind _order (`self.Order`))
  (bind _burger_ (`self.burger?`))
  (bind _cheeseburger (`self.CheeseBurger`))
  (bind _order_2 (`self.Order`))
  (bind _pizza_ (`self.Pizza?`))
  (bind _pizzapaprika_ (`self.PizzaPaprika?`))
  (bind _burger (`/Game/Cproef/Blueprints/AI/BP_AIOrder.Burger` _order_2))
  (bind _cheese (`/Game/Cproef/Blueprints/AI/BP_AIOrder.Cheese` _order_2))
  (bind _pizza (`/Game/Cproef/Blueprints/AI/BP_AIOrder.Pizza` _order))
  (bind _pizzaveg (`/Game/Cproef/Blueprints/AI/BP_AIOrder.PizzaVeg` _order))
  (`/Engine/EditorBlueprintResources/StandardMacros.IsValid` _order_2
    (:`Is Valid`
      (set `self.FoodScore` (`/Game/Cproef/Blueprints/AI/BP_AIOrder.AnotherScoreCauseFuckUnreal` _order_2))
      (if _burger_
        (if (and _burger_ _burger)
          (set `self.AITotalScore` (+ (`self.FoodScore`) 5))
          (elif (and (`self.burger?`) _cheese)
            (set `self.AITotalScore` (+ (`self.FoodScore`) 0))
            (else
              (set `self.AITotalScore` (- (`self.FoodScore`) 5)))))
        (`self.GradeHappiness`)
        (elif _cheeseburger
          (if (and _cheeseburger _cheese)
            (set `self.AITotalScore` (+ (`self.FoodScore`) 5))
            (elif (and _burger (`self.CheeseBurger`))
              (set `self.AITotalScore` (+ (`self.FoodScore`) 0))
              (else
                (set `self.AITotalScore` (- (`self.FoodScore`) 5)))))
          (`self.GradeHappiness`)
          (elif _pizza_
            (if (and _pizza_ _pizza)
              (set `self.AITotalScore` (+ (`self.FoodScore`) 5))
              (elif (and (`self.Pizza?`) _pizzaveg)
                (set `self.AITotalScore` (+ (`self.FoodScore`) 0))
                (else
                  (set `self.AITotalScore` (- (`self.FoodScore`) 5)))))
            (`self.GradeHappiness`)
            (elif _pizzapaprika_
              (if (and _pizzapaprika_ _pizzaveg)
                (set `self.AITotalScore` (+ (`self.FoodScore`) 5))
                (elif (and _pizzapaprika_ _pizza)
                  (set `self.AITotalScore` (+ (`self.FoodScore`) 0))
                  (else
                    (set `self.AITotalScore` (- (`self.FoodScore`) 5)))))
              (`self.GradeHappiness`))))))))

(event `self.CheckFood.OnComponentBeginOverlap`
  (params (OverlappedComponent :type "PrimitiveComponent Object Reference") (OtherActor :type "Actor Object Reference") (OtherComp :type "PrimitiveComponent Object Reference") (OtherBodyIndex :type Integer) (bFromSweep :type Boolean) (SweepResult :type "HitResult Structure (by ref)"))
  (bind _waypoints (`self.Waypoints`))
  (cast `/Game/Cproef/Blueprints/Cooking/BP_BurgerV2` OtherActor
    (:`then`
      _)
    (:`CastFailed`
      (cast `/Game/Cproef/Blueprints/Cooking/BP_PizzaV2` OtherActor
        (:`then`
          _)
        (:`CastFailed`
          (cast `/Game/Cproef/Blueprints/Cooking/BP_Plate` OtherActor
            (:`then`
              _)
            (:`CastFailed`
              (cast `/Game/Cproef/Blueprints/Cooking/BP_toppings` OtherActor)))))))
  (set `self.Angrery?` true)
  (`KismetSystemLibrary.Delay` 2.5)
  ;[1 1 1] Makes AI leave if to long in waiting line
  (`|AIMoveTo` self (0.0 0.0 0.0) (`/Game/Cproef/Blueprints/AI/BP_WaypointSystem.Waypoint4` _waypoints)
    (:`OnSuccess`
      (`KismetSystemLibrary.Delay` 0.05)
      (`|AIMoveTo` self (0.0 0.0 0.0) (`/Game/Cproef/Blueprints/AI/BP_WaypointSystem.Waypoint5` _waypoints)
        (:`OnSuccess`
          (`KismetSystemLibrary.Delay` 0.05)
          (`|AIMoveTo` self (0.0 0.0 0.0) (`/Game/Cproef/Blueprints/AI/BP_WaypointSystem.Waypoint6` _waypoints)
            (:`OnSuccess`
              (`self.K2_DestroyActor`))))))))

(fn `AttachPlate`
  (params (AttachParent :type "SceneComponent Object Reference") (Plate :type "/Game/Cproef/Blueprints/Cooking/BP_Plate Object Reference"))
  (`/Game/Cproef/Blueprints/Cooking/BP_Plate.AttachToAI` Plate AttachParent))

(fn `GradeHappiness`
  (bind _aitotalscore (`self.AITotalScore`))
  (if (>= _aitotalscore 14)
    (set `self.Happy?` true)
    (elif (`KismetMathLibrary.InRange_IntInt` _aitotalscore 8 13)
      (set `self.Neutral?` true)
      (elif (<= _aitotalscore 7)
        (set `self.Angrery?` true)))))

(fn `UserConstructionScript`
  (bind _returnvalue (`KismetMathLibrary.RandomInteger` 18))
  (bind _mesh (`self.Mesh`))
  (bind _mesh_2 (`self.Mesh`))
  (bind _mesh_3 (`self.Mesh`))
  (bind _mesh_4 (`self.Mesh`))
  (bind _mesh_5 (`self.Mesh`))
  (bind _mesh_6 (`self.Mesh`))
  (if (== _returnvalue 0)
    (`SkinnedMeshComponent.SetSkinnedAssetAndUpdate` _mesh_3 "/Game/Cproef/Models/AI/AI1/AI_Glasses.AI_Glasses" true)
    (elif (== _returnvalue 0)
      (`SkinnedMeshComponent.SetSkinnedAssetAndUpdate` _mesh_3 "/Game/Cproef/Models/AI/AI2/AI_Glasses_Hat.AI_Glasses_Hat" true)
      (elif (== _returnvalue 0)
        (`SkinnedMeshComponent.SetSkinnedAssetAndUpdate` _mesh_3 "/Game/Cproef/Models/AI/AI3/AI_Glasses_Mohawk.AI_Glasses_Mohawk" true)
        (elif (== _returnvalue 0)
          (`SkinnedMeshComponent.SetSkinnedAssetAndUpdate` _mesh_4 "/Game/Cproef/Models/AI/AI4/AI_Glasses_PoliceHat.AI_Glasses_PoliceHat" true)
          (elif (== _returnvalue 0)
            (`SkinnedMeshComponent.SetSkinnedAssetAndUpdate` _mesh_4 "/Game/Cproef/Models/AI/AI5/AI_Glasses_Sunhat.AI_Glasses_Sunhat" true)
            (elif (== _returnvalue 0)
              (`SkinnedMeshComponent.SetSkinnedAssetAndUpdate` _mesh_4 "/Game/Cproef/Models/AI/AI6/AI_Glasses_Tophat.AI_Glasses_Tophat" true)
              (elif (== _returnvalue 0)
                (`SkinnedMeshComponent.SetSkinnedAssetAndUpdate` _mesh_5 "/Game/Cproef/Models/AI/AI_Monocle/AI1/AI_Monocle.AI_Monocle" true)
                (elif (== _returnvalue 0)
                  (`SkinnedMeshComponent.SetSkinnedAssetAndUpdate` _mesh_5 "/Game/Cproef/Models/AI/AI_Monocle/AI2/AI_Monocle_Hat.AI_Monocle_Hat" true)
                  (elif (== _returnvalue 0)
                    (`SkinnedMeshComponent.SetSkinnedAssetAndUpdate` _mesh_5 "/Game/Cproef/Models/AI/AI_Monocle/AI_Monocle_Mohawk.AI_Monocle_Mohawk" true)
                    (elif (== _returnvalue 0)
                      (`SkinnedMeshComponent.SetSkinnedAssetAndUpdate` _mesh_6 "/Game/Cproef/Models/AI/AI_Monocle/AI_Monocle_PoliceHat.AI_Monocle_PoliceHat" true)
                      (elif (== _returnvalue 0)
                        (`SkinnedMeshComponent.SetSkinnedAssetAndUpdate` _mesh_6 "/Game/Cproef/Models/AI/AI_Monocle/AI_Monocle_SunHat.AI_Monocle_SunHat" true)
                        (elif (== _returnvalue 0)
                          (`SkinnedMeshComponent.SetSkinnedAssetAndUpdate` _mesh_6 "/Game/Cproef/Models/AI/AI_Monocle/AI_Monocle_TopHat.AI_Monocle_TopHat" true)
                          (elif (== _returnvalue 0)
                            (`SkinnedMeshComponent.SetSkinnedAssetAndUpdate` _mesh_2 "/Game/Cproef/Models/AI/AI_SunGlasses/AI1/AI_Sunglasses.AI_Sunglasses" true)
                            (elif (== _returnvalue 0)
                              (`SkinnedMeshComponent.SetSkinnedAssetAndUpdate` _mesh_2 "/Game/Cproef/Models/AI/AI_SunGlasses/AI2/AI_Sunglasses_Hat.AI_Sunglasses_Hat" true)
                              (elif (== _returnvalue 0)
                                (`SkinnedMeshComponent.SetSkinnedAssetAndUpdate` _mesh_2 "/Game/Cproef/Models/AI/AI_SunGlasses/AI3/AI_Sunglasses_Mohawk.AI_Sunglasses_Mohawk" true)
                                (elif (== _returnvalue 0)
                                  (`SkinnedMeshComponent.SetSkinnedAssetAndUpdate` _mesh "/Game/Cproef/Models/AI/AI_SunGlasses/AI4/AI_SunGlasses_PoliceHat.AI_SunGlasses_PoliceHat" true)
                                  (elif (== _returnvalue 0)
                                    (`SkinnedMeshComponent.SetSkinnedAssetAndUpdate` _mesh "/Game/Cproef/Models/AI/AI_SunGlasses/AI5/AI_Sunglasses_SunHat.AI_Sunglasses_SunHat" true)
                                    (elif (== _returnvalue 0)
                                      (`SkinnedMeshComponent.SetSkinnedAssetAndUpdate` _mesh "/Game/Cproef/Models/AI/AI_SunGlasses/AI6/AI_SunGlasses_TopHat.AI_SunGlasses_TopHat" true))))))))))))))))))))