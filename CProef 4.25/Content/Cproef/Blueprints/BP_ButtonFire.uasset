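; BP_ButtonFire is a physically pressable button that tells its parent BP_ToppingDispenser actor to spawn a topping.
; It tracks the first overlapping component and, each tick, converts that component's movement since overlap into a clamped press depth along the button's local Z axis.
; Reaching full depth fires SpawnTopping once until that component leaves.
; With nothing tracked, the button interpolates back to its starting position.
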(event `self.ReceiveBeginPlay`
  ;[1 1 1] Saving Start location of button
  (set `self.InitialButtonLocation` (`SceneComponent.RelativeLocation` (`self.Button`))))

(event `self.Button.OnComponentBeginOverlap`
  (params (OverlappedComponent :type "PrimitiveComponent Object Reference") (OtherActor :type "Actor Object Reference") (OtherComp :type "PrimitiveComponent Object Reference") (OtherBodyIndex :type Integer) (bFromSweep :type Boolean) (SweepResult :type "HitResult Structure (by ref)"))
  ;[1 1 1] Check if variable is empty
  (`/Engine/EditorBlueprintResources/StandardMacros.IsValid` (`self.OverlappedComponent`)
    (:`Is Not Valid`
      ;[1 1 1] If variable is empty, set the variable with the overlapped compinent and save the location of the initial overlap
      (bind _output_get (set `self.OverlappedComponent` OtherComp))
      (set `self.InitialOverlapLocation` (`SceneComponent.K2_GetComponentLocation` _output_get)))))

(event `self.Button.OnComponentEndOverlap`
  (params (OverlappedComponent :type "PrimitiveComponent Object Reference") (OtherActor :type "Actor Object Reference") (OtherComp :type "PrimitiveComponent Object Reference") (OtherBodyIndex :type Integer))
  ;[1 1 1] Check if component leaving overlap is the same as the one we're tracking
  (if (== OtherComp (`self.OverlappedComponent`))
    ;[1 1 1] If so clear the variable and change the color of the button
    (set `self.OverlappedComponent` null)
    (set `self.HasPressed` false)))

(event `self.ReceiveTick`
  (params (DeltaSeconds :type "Float (single-precision)"))
  (bind _button (`self.Button`))
  (bind (_returnvalue_x _returnvalue_y _returnvalue_z) (`KismetMathLibrary.BreakVector` (- (`KismetMathLibrary.InverseTransformDirection` (`SceneComponent.K2_GetComponentToWorld` _button) (`self.InitialOverlapLocation`)) (`KismetMathLibrary.InverseTransformDirection` (`SceneComponent.K2_GetComponentToWorld` _button) (`SceneComponent.K2_GetComponentLocation` (`self.OverlappedComponent`))))))
  (`/Engine/EditorBlueprintResources/StandardMacros.IsValid` (`self.OverlappedComponent`)
    (:`Is Valid`
      ;[1 1 1] Calculating the distance the button has been pressed and saving the distance
      (bind _output_get (set `self.SetButtonPressAmount` (`KismetMathLibrary.FClamp` _returnvalue_z 0.0 (`self.MaxButtonPress`))))
      ;[1 1 1] Updating button location with calculated value
      (`SceneComponent.K2_SetRelativeLocation` (`self.Button`) (- (`self.InitialButtonLocation`) (`KismetMathLibrary.MakeVector` 0.0 0.0 _output_get)) false false)
      ;[1 1 1] Check if we reached max button press
      (if (>= (`self.SetButtonPressAmount`) (`self.MaxButtonPress`))
        (if (not (`self.HasPressed`))
          (set `self.HasPressed` true)
          (bind _asbp_topping_dispenser (cast `/Game/Cproef/Blueprints/Cooking/BP_ToppingDispenser` (`self.GetParentActor`)))
          (`/Game/Cproef/Blueprints/Cooking/BP_ToppingDispenser.SpawnTopping` _asbp_topping_dispenser))))
    (:`Is Not Valid`
      ;[1 1 1] Return button to start location if overlapped component is empty
      (`SceneComponent.K2_SetRelativeLocation` (`self.Button`) (`KismetMathLibrary.VInterpTo` (`SceneComponent.RelativeLocation` (`self.Button`)) (`self.InitialButtonLocation`) DeltaSeconds 10.0) false false))))

(fn `UserConstructionScript`)