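; Customer AI character that queues at waypoints, orders a random burger or pizza variant, and grades the food it receives.
; It advances through three BP_WaypointSystem spots by polling occupancy, leaving and destroying itself after repeated blocked checks.
; At the front it shows the order on a material-swapped plane.
; Pickup attaches the plate and walks it away; happiness grading compares the order against BP_AIOrder, refetched every Tick, into Happy, Neutral or Angrery.
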(event `self.ReceiveTick`
  (params (DeltaSeconds :type "Float (single-precision)"))
  (bind _returnvalue (`GameplayStatics.GetActorOfClass` "/Game/Cproef/Blueprints/AI/BP_AIOrder.BP_AIOrder_C"))
  (set `self.Order` _returnvalue))

(event `InitiateActor`
  (bind _returnvalue (`GameplayStatics.GetActorOfClass` "/Game/Cproef/Blueprints/AI/BP_WaypointSystem.BP_WaypointSystem_C"))
  (set `self.Waypoints` _returnvalue)
  (`self.WaitingLine`))

(event `self.ReceiveBeginPlay`
  (`self.InitiateActor`)
  (`SceneComponent.SetVisibility` (`self.Plane`) false false))

(event `WaitingLine`
  (bind _waypoints (`self.Waypoints`))
  (bind _waypoints_2 (`self.Waypoints`))
  (if (`/Game/Cproef/Blueprints/AI/BP_WaypointSystem.Spot3Filled?` (`self.Waypoints`)) :!label _label
    (`KismetSystemLibrary.Delay` 5.0)
    (goto _label)
    (else
      ;[1 1 1] Moves AI to 3spot in waiting line
      (`|AIMoveTo` self (0.0 0.0 0.0) (`/Game/Cproef/Blueprints/AI/BP_WaypointSystem.Waypoint3` (`self.Waypoints`))
        (:`OnSuccess`
          (`KismetSystemLibrary.Delay` 0.2)
          ;[1 1 1] checks if next spot is free to move too
          (if (`/Game/Cproef/Blueprints/AI/BP_WaypointSystem.Spot2Filled?` (`self.Waypoints`)) :!label _label_2
            ;[1 1 1] checks how long the AI has been waiting without moving
            (bind _output_get (set `self.delayFrequenty?` (+ (`self.delayFrequenty?`) 1.0)))
            (if (>= _output_get 3.0)
              ;[1 1 1] Makes AI leave if to long in waiting line
              (`|AIMoveTo` self (0.0 0.0 0.0) (`/Game/Cproef/Blueprints/AI/BP_WaypointSystem.Waypoint4` _waypoints)
                (:`OnSuccess`
                  (`KismetSystemLibrary.Delay` 0.05)
                  (`|AIMoveTo` self (0.0 0.0 0.0) (`/Game/Cproef/Blueprints/AI/BP_WaypointSystem.Waypoint5` _waypoints)
                    (:`OnSuccess`
                      (`KismetSystemLibrary.Delay` 0.05)
                      (`|AIMoveTo` self (0.0 0.0 0.0) (`/Game/Cproef/Blueprints/AI/BP_WaypointSystem.Waypoint6` _waypoints)
                        (:`OnSuccess`
                          (`self.K2_DestroyActor`)))))))
              (else
                (`KismetSystemLibrary.Delay` 5.0)
                (goto _label_2)))
            (else
              (`|AIMoveTo` self (0.0 0.0 0.0) (`/Game/Cproef/Blueprints/AI/BP_WaypointSystem.Waypoint2` (`self.Waypoints`))
                (:`OnSuccess`
                  (`KismetSystemLibrary.Delay` 0.2)
                  (if (`/Game/Cproef/Blueprints/AI/BP_WaypointSystem.Spot1Filled?` (`self.Waypoints`)) :!label _label_3
                    (bind _output_get_2 (set `self.delayFrequenty?` (+ (`self.delayFrequenty?`) 1.0)))
                    (if (>= _output_get_2 3.0)
                      ;[1 1 1] Makes AI leave if to long in waiting line
                      (`|AIMoveTo` self (0.0 0.0 0.0) (`/Game/Cproef/Blueprints/AI/BP_WaypointSystem.Waypoint4` _waypoints_2)
                        (:`OnSuccess`
                          (`|AIMoveTo` self (0.0 0.0 0.0) (`/Game/Cproef/Blueprints/AI/BP_WaypointSystem.Waypoint5` _waypoints_2)
                            (:`OnSuccess`
                              (`|AIMoveTo` self (0.0 0.0 0.0) (`/Game/Cproef/Blueprints/AI/BP_WaypointSystem.Waypoint6` _waypoints_2)
                                (:`OnSuccess`
                                  (`self.K2_DestroyActor`)))))))
                      (else
                        (`KismetSystemLibrary.Delay` 5.0)
                        (goto _label_3)))
                    (else
                      (`|AIMoveTo` self (0.0 0.0 0.0) (`/Game/Cproef/Blueprints/AI/BP_WaypointSystem.Waypoint1` (`self.Waypoints`))
                        (:`OnSuccess`
                          ;[1 1 1] AI can order here
                          (set `self.canOrder?` true)
                          (`self.Ordering`)
                          (set `self.ordered?` true)
                          (`SceneComponent.SetVisibility` (`self.Plane`) true false))))))))))))))

(event `Ordering`
  ;[1 1 1] generationg a random int and checking the value
  (switch `int` (`KismetMathLibrary.RandomInteger` (enumcount `/Game/Cproef/Blueprints/AI/Enum_Orders`))
    (:`Default`
      ;[1 1 1] just to fill up false, should never happen.. normally..
      (`KismetSystemLibrary.PrintString` "welp unlucky"))
    (:`0`
      ;[1 1 1] determing what to order depending on the randomly generated int
      (set `self.burger?` true)
      (`PrimitiveComponent.SetMaterial` (`self.Plane`) 0 "/Game/Cproef/Textures/M_OrderBurger.M_OrderBurger"))
    (:`1`
      (set `self.CheeseBurger` true)
      (`PrimitiveComponent.SetMaterial` (`self.Plane`) 0 "/Game/Cproef/Textures/M_OrderCheeseBurger.M_OrderCheeseBurger"))
    (:`2`
      (set `self.Pizza?` true)
      (`PrimitiveComponent.SetMaterial` (`self.Plane`) 0 "/Game/Cproef/Textures/M_OrderPizzaSalami.M_OrderPizzaSalami"))
    (:`3`
      (set `self.PizzaPaprika?` true)
      (`PrimitiveComponent.SetMaterial` (`self.Plane`) 0 "/Game/Cproef/Textures/M_OrderPizzaVeggie.M_OrderPizzaVeggie"))))

(event `FoodPickUp`
  (params (PlateToPickup :type "/Game/Cproef/Blueprints/Cooking/BP_Plate Object Reference"))
  (`KismetSystemLibrary.Delay` 0.5)
  (`self.AttachPlate` (`self.FoodHolder`) PlateToPickup)
  (`PrimitiveComponent.SetCollisionEnabled` (`StaticMeshActor.StaticMeshComponent` PlateToPickup) "NoCollision")
  (`KismetSystemLibrary.Delay` 1.0)
  (`self.Happiness?`)
  (`SceneComponent.SetVisibility` (`self.Plane`) false false)
  (`|AIMoveTo` self (0.0 0.0 0.0) (`/Game/Cproef/Blueprints/AI/BP_WaypointSystem.Waypoint4` (`self.Waypoints`))
    (:`OnSuccess`
      (`|AIMoveTo` self (0.0 0.0 0.0) (`/Game/Cproef/Blueprints/AI/BP_WaypointSystem.Waypoint5` (`self.Waypoints`))
        (:`OnSuccess`
          (`|AIMoveTo` self (0.0 0.0 0.0) (`/Game/Cproef/Blueprints/AI/BP_WaypointSystem.Waypoint7` (`self.Waypoints`))))))))

(event `AcceptedOrder`)

(event `Happiness?`
  (bind _order (`self.Order`))
  (bind _burger_ (`self.burger?`))
  (bind _cheeseburger (`self.CheeseBurger`))
  (bind _order_2 (`self.Order`))
  (bind _pizza_ (`self.Pizza?`))
  (bind _pizzapaprika_ (`self.PizzaPaprika?`))
  (bind _burger (`/Game/Cproef/Blueprints/AI/BP_AIOrder.Burger` _order_2))
  (bind _cheese (`/Game/Cproef/Blueprints/AI/BP_AIOrder.Cheese` _order_2))
  (bind _pizza (`/Game/Cproef/Blueprints/AI/BP_AIOrder.Pizza` _order))
  (bind _pizzaveg (`/Game/Cproef/Blueprints/AI/BP_AIOrder.PizzaVeg` _order))
  (`/Engine/EditorBlueprintResources/StandardMacros.IsValid` _order_2
    (:`Is Valid`
      (set `self.FoodScore` (`/Game/Cproef/Blueprints/AI/BP_AIOrder.AnotherScoreCauseFuckUnreal` _order_2))
      (if _burger_
        (if (and _burger_ _burger)
          (set `self.AITotalScore` (+ (`self.FoodScore`) 5))
          (elif (and (`self.burger?`) _cheese)
            (set `self.AITotalScore` (+ (`self.FoodScore`) 0))
            (else
              (set `self.AITotalScore` (- (`self.FoodScore`) 5)))))
        (`self.GradeHappiness`)
        (elif _cheeseburger
          (if (and _cheeseburger _cheese)
            (set `self.AITotalScore` (+ (`self.FoodScore`) 5))
            (elif (and _burger (`self.CheeseBurger`))
              (set `self.AITotalScore` (+ (`self.FoodScore`) 0))
              (else
                (set `self.AITotalScore` (- (`self.FoodScore`) 5)))))
          (`self.GradeHappiness`)
          (elif _pizza_
            (if (and _pizza_ _pizza)
              (set `self.AITotalScore` (+ (`self.FoodScore`) 5))
              (elif (and (`self.Pizza?`) _pizzaveg)
                (set `self.AITotalScore` (+ (`self.FoodScore`) 0))
                (else
                  (set `self.AITotalScore` (- (`self.FoodScore`) 5)))))
            (`self.GradeHappiness`)
            (elif _pizzapaprika_
              (if (and _pizzapaprika_ _pizzaveg)
                (set `self.AITotalScore` (+ (`self.FoodScore`) 5))
                (elif (and _pizzapaprika_ _pizza)
                  (set `self.AITotalScore` (+ (`self.FoodScore`) 0))
                  (else
                    (set `self.AITotalScore` (- (`self.FoodScore`) 5)))))
              (`self.GradeHappiness`))))))))

(fn `AttachPlate`
  (params (AttachParent :type "SceneComponent Object Reference") (Plate :type "/Game/Cproef/Blueprints/Cooking/BP_Plate Object Reference"))
  (`/Game/Cproef/Blueprints/Cooking/BP_Plate.AttachToAI` Plate AttachParent))

(fn `GradeHappiness`
  (bind _aitotalscore (`self.AITotalScore`))
  (if (>= _aitotalscore 14)
    (set `self.Happy?` true)
    (elif (`KismetMathLibrary.InRange_IntInt` _aitotalscore 8 13)
      (set `self.Neutral?` true)
      (elif (<= _aitotalscore 7)
        (set `self.Angrery?` true)))))

(fn `UserConstructionScript`)