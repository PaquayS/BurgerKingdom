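; Spawner actor that creates BP_AIChar01 AI characters at its SpawnArea component when its Spawn event is called.
; Each call spawns one character through SpawnAIFromClass, runs its InitiateActor and increments AIsSpawned, up to a cap of four.
; The counter is never decremented here, and the GetAllActorsOfClass result is unused.
; Tick is empty, and a leftover SpawnActor node is disconnected.
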(event `self.ReceiveTick`
  (params (DeltaSeconds :type "Float (single-precision)")))

(event `Spawn`
  (`GameplayStatics.GetAllActorsOfClass` "/Game/Cproef/test/BP_AIChar01.BP_AIChar01_C")
  (if (< (`self.AIsSpawned`) 4)
    (bind _returnvalue (`AIBlueprintHelperLibrary.SpawnAIFromClass` "/Game/Cproef/test/BP_AIChar01.BP_AIChar01_C" null (`SceneComponent.K2_GetComponentLocation` (`self.SpawnArea`))))
    (bind _asbp_aichar_01 (cast `/Game/Cproef/test/BP_AIChar01` _returnvalue))
    (`/Game/Cproef/test/BP_AIChar01.InitiateActor` _asbp_aichar_01)
    (bind _result (`/Engine/EditorBlueprintResources/StandardMacros.IncrementInt` (`self.AIsSpawned`))
      (:`  `
        (set `self.AIsSpawned` _result)))))

(fn `UserConstructionScript`)