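; BP_AIOrder is a pickup zone that hands plates placed in its box to AI customers who have ordered.
; Tick rebuilds the BP_AIChar01 list every frame, overwriting any AddNewAI additions.
; On overlap, every customer flagged Ordered receives FoodPickUp with the plate, whose score and food type (burger, cheese or pizza variants) are recorded.
; The logic paying price and tip into the MotionControllerPawn's wallet is disconnected.
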(event `self.ReceiveTick`
  (params (DeltaSeconds :type "Float (single-precision)"))
  (bind _outactors (`GameplayStatics.GetAllActorsOfClass` "/Game/Cproef/test/BP_AIChar01.BP_AIChar01_C"))
  (set `self.AI` _outactors))

(event `self.ReceiveBeginPlay`)

(event `AddNewAI`
  (params (NewParam :type "/Game/Cproef/test/BP_AIChar01 Object Reference"))
  (`KismetArrayLibrary.Array_Add` (`self.AI`) NewParam))

(event `self.Box.OnComponentBeginOverlap`
  (params (OverlappedComponent :type "PrimitiveComponent Object Reference") (OtherActor :type "Actor Object Reference") (OtherComp :type "PrimitiveComponent Object Reference") (OtherBodyIndex :type Integer) (bFromSweep :type Boolean) (SweepResult :type "HitResult Structure (by ref)"))
  (bind _pickupplateforcustomer (`self.PickUpPlateForCustomer`))
  (bind _asbp_plate (cast `/Game/Cproef/Blueprints/Cooking/BP_Plate` OtherActor))
  (set `self.PickUpPlateForCustomer` _asbp_plate)
  (for _array_element (`self.AI`)
    (if (`/Game/Cproef/test/BP_AIChar01.ordered?` _array_element)
      (`/Game/Cproef/test/BP_AIChar01.FoodPickUp` _array_element (`self.PickUpPlateForCustomer`))
      (bind _returnvalue (`GameplayStatics.GetActorOfClass` "/Game/VirtualRealityBP/Blueprints/MotionControllerPawn.MotionControllerPawn_C"))
      (set `self.AnotherScoreCauseFuckUnreal` (`/Game/Cproef/Blueprints/Cooking/BP_Plate.TotalScore` _asbp_plate))
      (if (`/Game/Cproef/Blueprints/Cooking/BP_Plate.B?` _pickupplateforcustomer)
        (set `self.Burger` true)
        (elif (`/Game/Cproef/Blueprints/Cooking/BP_Plate.CB?` _pickupplateforcustomer)
          (set `self.Cheese` true)
          (elif (`/Game/Cproef/Blueprints/Cooking/BP_Plate.PS?` _pickupplateforcustomer)
            (set `self.Pizza` true)
            (elif (`/Game/Cproef/Blueprints/Cooking/BP_Plate.PV?` _pickupplateforcustomer)
              (set `self.PizzaVeg` true))))))))

(event `self.Box.OnComponentEndOverlap`
  (params (OverlappedComponent :type "PrimitiveComponent Object Reference") (OtherActor :type "Actor Object Reference") (OtherComp :type "PrimitiveComponent Object Reference") (OtherBodyIndex :type Integer))
  (cast `/Game/Cproef/Blueprints/Cooking/BP_Plate` OtherActor)
  (set `self.PickUpPlateForCustomer` null))

(fn `UserConstructionScript`)