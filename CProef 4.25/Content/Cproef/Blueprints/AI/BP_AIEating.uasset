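; AI eating character whose shown logic only randomizes its appearance, picking a skeletal mesh variant with different eyewear and headwear.
; The Construction Script runs a nested chain of independent 1-in-18 rolls, so earlier variants are likelier and the default mesh remains if all rolls fail.
; The event graph holds only disabled placeholder events, so no eating or AI behavior is implemented there.
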(fn `UserConstructionScript`
  (bind _returnvalue (`KismetMathLibrary.RandomInteger` 18))
  (bind _skeletalmesh (`self.SkeletalMesh`))
  (bind _skeletalmesh_2 (`self.SkeletalMesh`))
  (bind _skeletalmesh_3 (`self.SkeletalMesh`))
  (bind _skeletalmesh_4 (`self.SkeletalMesh`))
  (bind _skeletalmesh_5 (`self.SkeletalMesh`))
  (bind _skeletalmesh_6 (`self.SkeletalMesh`))
  (if (== _returnvalue 0)
    (`SkinnedMeshComponent.SetSkinnedAssetAndUpdate` _skeletalmesh_3 "/Game/Cproef/Models/AI/AI1/AI_Glasses.AI_Glasses" true)
    (elif (== _returnvalue 0)
      (`SkinnedMeshComponent.SetSkinnedAssetAndUpdate` _skeletalmesh_3 "/Game/Cproef/Models/AI/AI2/AI_Glasses_Hat.AI_Glasses_Hat" true)
      (elif (== _returnvalue 0)
        (`SkinnedMeshComponent.SetSkinnedAssetAndUpdate` _skeletalmesh_3 "/Game/Cproef/Models/AI/AI3/AI_Glasses_Mohawk.AI_Glasses_Mohawk" true)
        (elif (== _returnvalue 0)
          (`SkinnedMeshComponent.SetSkinnedAssetAndUpdate` _skeletalmesh_4 "/Game/Cproef/Models/AI/AI4/AI_Glasses_PoliceHat.AI_Glasses_PoliceHat" true)
          (elif (== _returnvalue 0)
            (`SkinnedMeshComponent.SetSkinnedAssetAndUpdate` _skeletalmesh_4 "/Game/Cproef/Models/AI/AI5/AI_Glasses_Sunhat.AI_Glasses_Sunhat" true)
            (elif (== _returnvalue 0)
              (`SkinnedMeshComponent.SetSkinnedAssetAndUpdate` _skeletalmesh_4 "/Game/Cproef/Models/AI/AI6/AI_Glasses_Tophat.AI_Glasses_Tophat" true)
              (elif (== _returnvalue 0)
                (`SkinnedMeshComponent.SetSkinnedAssetAndUpdate` _skeletalmesh_5 "/Game/Cproef/Models/AI/AI_Monocle/AI1/AI_Monocle.AI_Monocle" true)
                (elif (== _returnvalue 0)
                  (`SkinnedMeshComponent.SetSkinnedAssetAndUpdate` _skeletalmesh_5 "/Game/Cproef/Models/AI/AI_Monocle/AI2/AI_Monocle_Hat.AI_Monocle_Hat" true)
                  (elif (== _returnvalue 0)
                    (`SkinnedMeshComponent.SetSkinnedAssetAndUpdate` _skeletalmesh_5 "/Game/Cproef/Models/AI/AI_Monocle/AI_Monocle_Mohawk.AI_Monocle_Mohawk" true)
                    (elif (== _returnvalue 0)
                      (`SkinnedMeshComponent.SetSkinnedAssetAndUpdate` _skeletalmesh_6 "/Game/Cproef/Models/AI/AI_Monocle/AI_Monocle_PoliceHat.AI_Monocle_PoliceHat" true)
                      (elif (== _returnvalue 0)
                        (`SkinnedMeshComponent.SetSkinnedAssetAndUpdate` _skeletalmesh_6 "/Game/Cproef/Models/AI/AI_Monocle/AI_Monocle_SunHat.AI_Monocle_SunHat" true)
                        (elif (== _returnvalue 0)
                          (`SkinnedMeshComponent.SetSkinnedAssetAndUpdate` _skeletalmesh_6 "/Game/Cproef/Models/AI/AI_Monocle/AI_Monocle_TopHat.AI_Monocle_TopHat" true)
                          (elif (== _returnvalue 0)
                            (`SkinnedMeshComponent.SetSkinnedAssetAndUpdate` _skeletalmesh_2 "/Game/Cproef/Models/AI/AI_SunGlasses/AI1/AI_Sunglasses.AI_Sunglasses" true)
                            (elif (== _returnvalue 0)
                              (`SkinnedMeshComponent.SetSkinnedAssetAndUpdate` _skeletalmesh_2 "/Game/Cproef/Models/AI/AI_SunGlasses/AI2/AI_Sunglasses_Hat.AI_Sunglasses_Hat" true)
                              (elif (== _returnvalue 0)
                                (`SkinnedMeshComponent.SetSkinnedAssetAndUpdate` _skeletalmesh_2 "/Game/Cproef/Models/AI/AI_SunGlasses/AI3/AI_Sunglasses_Mohawk.AI_Sunglasses_Mohawk" true)
                                (elif (== _returnvalue 0)
                                  (`SkinnedMeshComponent.SetSkinnedAssetAndUpdate` _skeletalmesh "/Game/Cproef/Models/AI/AI_SunGlasses/AI4/AI_SunGlasses_PoliceHat.AI_SunGlasses_PoliceHat" true)
                                  (elif (== _returnvalue 0)
                                    (`SkinnedMeshComponent.SetSkinnedAssetAndUpdate` _skeletalmesh "/Game/Cproef/Models/AI/AI_SunGlasses/AI5/AI_Sunglasses_SunHat.AI_Sunglasses_SunHat" true)
                                    (elif (== _returnvalue 0)
                                      (`SkinnedMeshComponent.SetSkinnedAssetAndUpdate` _skeletalmesh "/Game/Cproef/Models/AI/AI_SunGlasses/AI6/AI_SunGlasses_TopHat.AI_SunGlasses_TopHat" true))))))))))))))))))))