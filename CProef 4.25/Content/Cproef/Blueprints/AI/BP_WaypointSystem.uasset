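; Waypoint system actor that tracks which of three spots are occupied by BP_AIChar01 characters.
; Each of three box triggers sets its SpotFilled flag when such a character begins overlapping and clears it when one leaves.
; Entering the first or second box also clears the following spot's flag.
; The flags are simple booleans with no occupant counting, and this graph only writes them.
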(event `self.Box.OnComponentBeginOverlap`
  (params (OverlappedComponent :type "PrimitiveComponent Object Reference") (OtherActor :type "Actor Object Reference") (OtherComp :type "PrimitiveComponent Object Reference") (OtherBodyIndex :type Integer) (bFromSweep :type Boolean) (SweepResult :type "HitResult Structure (by ref)"))
  (cast `/Game/Cproef/test/BP_AIChar01` OtherActor)
  (set `self.Spot1Filled?` true)
  (set `self.Spot2Filled?` false))

(event `self.Box1.OnComponentBeginOverlap`
  (params (OverlappedComponent :type "PrimitiveComponent Object Reference") (OtherActor :type "Actor Object Reference") (OtherComp :type "PrimitiveComponent Object Reference") (OtherBodyIndex :type Integer) (bFromSweep :type Boolean) (SweepResult :type "HitResult Structure (by ref)"))
  (cast `/Game/Cproef/test/BP_AIChar01` OtherActor)
  (set `self.Spot2Filled?` true)
  (set `self.Spot3Filled?` false))

(event `self.Box2.OnComponentBeginOverlap`
  (params (OverlappedComponent :type "PrimitiveComponent Object Reference") (OtherActor :type "Actor Object Reference") (OtherComp :type "PrimitiveComponent Object Reference") (OtherBodyIndex :type Integer) (bFromSweep :type Boolean) (SweepResult :type "HitResult Structure (by ref)"))
  (cast `/Game/Cproef/test/BP_AIChar01` OtherActor)
  (set `self.Spot3Filled?` true))

(event `self.Box.OnComponentEndOverlap`
  (params (OverlappedComponent :type "PrimitiveComponent Object Reference") (OtherActor :type "Actor Object Reference") (OtherComp :type "PrimitiveComponent Object Reference") (OtherBodyIndex :type Integer))
  (cast `/Game/Cproef/test/BP_AIChar01` OtherActor)
  (set `self.Spot1Filled?` false))

(event `self.Box1.OnComponentEndOverlap`
  (params (OverlappedComponent :type "PrimitiveComponent Object Reference") (OtherActor :type "Actor Object Reference") (OtherComp :type "PrimitiveComponent Object Reference") (OtherBodyIndex :type Integer))
  (cast `/Game/Cproef/test/BP_AIChar01` OtherActor)
  (set `self.Spot2Filled?` false))

(event `self.Box2.OnComponentEndOverlap`
  (params (OverlappedComponent :type "PrimitiveComponent Object Reference") (OtherActor :type "Actor Object Reference") (OtherComp :type "PrimitiveComponent Object Reference") (OtherBodyIndex :type Integer))
  (cast `/Game/Cproef/test/BP_AIChar01` OtherActor)
  (set `self.Spot3Filled?` false))

(fn `UserConstructionScript`)