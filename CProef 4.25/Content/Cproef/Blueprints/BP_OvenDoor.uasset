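; BP_OvenDoor is an oven door that swings open or closed when a VR motion controller or a plain StaticMeshActor overlaps its box.
; The DoorOpen flag selects one of two timelines that drive the mesh's world pitch, with CanInteract blocking retriggers until the swing finishes.
; Pickup and Drop store or clear an attach target, but the look-at rotation that reads it never runs.
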(event `self.ReceiveBeginPlay`
  (set `self.CanInteract?` true))

(event `/Game/VirtualRealityBP/Blueprints/PickupActorInterface.Pickup`
  (params (AttachTo :type "SceneComponent Object Reference"))
  (set `self.NewVar_1` AttachTo))

(event `/Game/VirtualRealityBP/Blueprints/PickupActorInterface.Drop`
  (set `self.NewVar_1` null))

(event `self.Box.OnComponentBeginOverlap`
  (params (OverlappedComponent :type "PrimitiveComponent Object Reference") (OtherActor :type "Actor Object Reference") (OtherComp :type "PrimitiveComponent Object Reference") (OtherBodyIndex :type Integer) (bFromSweep :type Boolean) (SweepResult :type "HitResult Structure (by ref)"))
  (if (`self.CanInteract?`)
    (cast `/Game/VirtualRealityBP/Blueprints/BP_MotionController` OtherActor
      (:`then`
        (set `self.CanInteract?` false)
        (if (`self.DoorOpen?`) :!label _label
          (bind (_direction _newtrack_0) (`Timeline|Open door` :!via `PlayFromStart`)
            (:`Update`
              (`SceneComponent.K2_SetWorldRotation` (`self.StaticMeshComponent`) (`KismetMathLibrary.MakeRotator` 0.0 _newtrack_0) false false))
            (:`Finished`
              (set `self.DoorOpen?` false)
              (set `self.CanInteract?` true)))
          (else
            (bind (_direction_2 _newtrack_0_2) (`Timeline|Timeline_0` :!via `PlayFromStart`)
              (:`Update`
                (`SceneComponent.K2_SetWorldRotation` (`self.StaticMeshComponent`) (`KismetMathLibrary.MakeRotator` 0.0 _newtrack_0_2) false false))
              (:`Finished`
                (set `self.DoorOpen?` true)
                (set `self.CanInteract?` true))))))
      (:`CastFailed`
        (if (== (`GameplayStatics.GetObjectClass` OtherActor) "/Script/Engine.StaticMeshActor")
          (set `self.CanInteract?` false)
          (goto _label))))))

(fn `UserConstructionScript`)