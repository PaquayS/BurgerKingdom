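; BP_TestVelocity is a test Blueprint that measures the speed of its static mesh component.
; BeginPlay records the starting world position and resets a running time value.
; Each Tick divides the change in world position by the elapsed frame time and stores the vector length as a scalar Velocity, then saves the current position and time for the next frame.
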(event `self.ReceiveBeginPlay`
  (set `self.PreviousPosition` (`SceneComponent.K2_GetComponentLocation` (`self.StaticMeshComponent`)))
  (set `self.PreviousTime` 0.0))

(event `self.ReceiveTick`
  (params (DeltaSeconds :type "Float (single-precision)"))
  (bind _output_get (set `self.CurrentTime` (+ (`self.PreviousTime`) DeltaSeconds)))
  (set `self.CurrentPosition` (`SceneComponent.K2_GetComponentLocation` (`self.StaticMeshComponent`)))
  (set `self.Velocity` (`KismetMathLibrary.VSize` (/ (- (`self.CurrentPosition`) (`self.PreviousPosition`)) (- _output_get (`self.PreviousTime`)))))
  (set `self.PreviousTime` (`self.CurrentTime`))
  (set `self.PreviousPosition` (`self.CurrentPosition`)))

(fn `UserConstructionScript`)