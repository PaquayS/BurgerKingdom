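; BP_Pizza is a motion-controller grabbable pizza that collects toppings and scores the prepared dish.
; ToppingDetector overlaps snap each BP_toppings actor onto the stack, raise the detector by its thickness, count it by type and add a cooking-state score.
; AttachToPlate attaches the pizza and adds a quantity score for pizza base, salami and paprika to the total.
; Topping removal is left unwired, and Drop disables the detector and keeps physics off.
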(event `/Game/VirtualRealityBP/Blueprints/PickupActorInterface.Pickup`
  (params (AttachTo :type "SceneComponent Object Reference"))
  (`PrimitiveComponent.SetSimulatePhysics` (`self.StaticMesh`) false)
  (`SceneComponent.K2_AttachToComponent` (`self.RootComponent`) AttachTo "None" "KeepWorld" "KeepWorld" "KeepWorld" false))

(event `/Game/VirtualRealityBP/Blueprints/PickupActorInterface.Drop`
  (`PrimitiveComponent.SetCollisionEnabled` (`self.ToppingDetector`) "NoCollision")
  (`PrimitiveComponent.SetSimulatePhysics` (`self.StaticMesh`) false)
  (`self.K2_DetachFromActor` "KeepWorld" "KeepWorld" "KeepWorld"))

(event `self.ToppingDetector.OnComponentBeginOverlap`
  (params (OverlappedComponent :type "PrimitiveComponent Object Reference") (OtherActor :type "Actor Object Reference") (OtherComp :type "PrimitiveComponent Object Reference") (OtherBodyIndex :type Integer) (bFromSweep :type Boolean) (SweepResult :type "HitResult Structure (by ref)"))
  (bind _currenttopping (`self.CurrentTopping`))
  (bind _currentoffset (`self.CurrentOffset`))
  ;[1 1 1] Setting current topping to know what topping you added
  (bind _asbp_toppings (cast `/Game/Cproef/Blueprints/Cooking/BP_toppings` OtherActor))
  (set `self.CurrentTopping` _asbp_toppings)
  (`/Engine/EditorBlueprintResources/StandardMacros.IsValid` _currenttopping
    (:`Is Valid`
      (set `/Game/Cproef/Blueprints/Cooking/BP_toppings.AttachedToBurger?` true _currenttopping)
      (`/Game/VirtualRealityBP/Blueprints/PickupActorInterface.Drop` _currenttopping)
      (`PrimitiveComponent.SetCollisionEnabled` (`StaticMeshActor.StaticMeshComponent` _currenttopping) "NoCollision")
      (`self.K2_AttachToActor` _currenttopping self "None" "SnapToTarget" "SnapToTarget" "KeepWorld" true)
      (`SceneComponent.K2_SetRelativeLocation` (`Actor.RootComponent` _currenttopping) (`KismetMathLibrary.MakeVector` 0.0 0.0 (- _currentoffset 0.75)) false true)
      (bind _output_get (set `self.CurrentOffset` (+ _currentoffset (`/Game/Cproef/Blueprints/Cooking/BP_toppings.Thiccness` _currenttopping))))
      (if (not (`self.RemovingTopping?`))
        (`self.IncreaseToppingsAmount`)
        (`self.AddToTotalScore`)
        (`KismetArrayLibrary.Array_Add` (`self.Toppings`) (`self.CurrentTopping`))
        (set `self.CurrentTopping` null)
        (`SceneComponent.K2_SetRelativeLocation` (`self.ToppingDetector`) (`KismetMathLibrary.MakeVector` 0.0 0.0 _output_get) false false)))))

(event `self.ReceiveTick`
  (params (DeltaSeconds :type "Float (single-precision)")))

(event `AttachToPlate`
  (params (PlateToAttachTo :type "/Game/Cproef/Blueprints/Cooking/BP_Plate Object Reference"))
  ;[1 1 1] Attach the food to the plate
  (`self.K2_AttachToActor` PlateToAttachTo "None" "KeepWorld" "KeepWorld" "KeepWorld")
  (`self.ToppingScore`)
  (bind _output_get (set `self.ScoreTot` (+ (`self.ScoreTop`) (`self.ScoreTot`)))))

(event `CookingScore`
  ;[1 1 1] Deciding how good the food has been cooked
  (if (`/Game/Cproef/Blueprints/Cooking/BP_toppings.raw?` (`self.CurrentTopping`))
    (set `self.ScoreC` 0.0)
    (elif (`/Game/Cproef/Blueprints/Cooking/BP_toppings.Cooked?` (`self.CurrentTopping`))
      (set `self.ScoreC` 10.0)
      (else
        (if (`/Game/Cproef/Blueprints/Cooking/BP_toppings.Burned?` (`self.CurrentTopping`))
          _
          (else
            _))
        (set `self.ScoreC` 5.0)))))

(event `RemoveFromTotalScore`)

(event `AddToTotalScore`
  ;[1 1 1] Setting total score of prepared dish
  (`self.CookingScore`)
  (set `self.ScoreTot` (+ (`self.ScoreTot`) (`self.ScoreC`))))

(event `ToppingScore`
  (bind _amountpaprika (`self.AmountPaprika`))
  (bind _amountsalami (`self.AmountSalami`))
  (bind _amountpd (`self.AmountPD`))
  ;[1 1 1] Topping Score for the BBuns
  (if (== _amountpd 0)
    (set `self.ScoreTop` (+ 0.0 (`self.ScoreTop`)))
    ;[1 1 1] Topping Score for amount of meat, because meat is good you're not punished for using double meat. BUT if you use more you'll get negative score
    (if (>= 5 _amountsalami) :!label _label
      (set `self.ScoreTop` (+ 0.0 (`self.ScoreTop`)))
      ;[1 1 1] scoring for cheese, same rules as meat
      (if (>= 5 _amountpaprika) :!label _label_2
        (set `self.ScoreTop` (+ 0.0 (`self.ScoreTop`)))
        (elif (`KismetMathLibrary.InRange_IntInt` _amountpaprika 6 14)
          (set `self.ScoreTop` (+ 10.0 (`self.ScoreTop`)))
          (elif (>= _amountpaprika 15)
            (set `self.ScoreTop` (+ (`self.ScoreTop`) (- 10.0 (* (- (`self.AmountPaprika`) 14) 0.5)))))))
      (elif (`KismetMathLibrary.InRange_IntInt` _amountsalami 6 14)
        (set `self.ScoreTop` (+ 10.0 (`self.ScoreTop`)))
        (goto _label_2)
        (elif (>= _amountsalami 15)
          (set `self.ScoreTop` (+ (`self.ScoreTop`) (- 10.0 (* (- (`self.AmountSalami`) 14) 0.5))))
          (goto _label_2))))
    (elif (== _amountpd 1)
      (set `self.ScoreTop` (+ 10.0 (`self.ScoreTop`)))
      (goto _label)
      (elif (>= _amountpd 2)
        (set `self.ScoreTop` (+ (`self.ScoreTop`) (- 10.0 (* (`self.AmountPD`) 5.0))))
        (goto _label)))))

(event `self.ReceiveBeginPlay`)

(fn `CalculateVelocity`
  (params (CurrentPosition :type "Vector Structure") (DeltaSeconds :type "Float (double-precision)"))
  (bind _output_get (set `self.CurrentTime` (+ (`self.PreviousTime`) DeltaSeconds)))
  (set `self.CurrentPosition` CurrentPosition)
  (set `self.Velocity` (`KismetMathLibrary.VSize` (/ (- (`self.CurrentPosition`) (`self.PreviousPosition`)) (- _output_get (`self.PreviousTime`)))))
  (set `self.PreviousTime` (`self.CurrentTime`))
  (set `self.PreviousPosition` (`self.CurrentPosition`)))

(fn `DecreaseToppingsAmount`
  (bind _returnvalue (`|GetEnumeratorNameAsString` (`/Game/Cproef/Blueprints/Cooking/BP_toppings.topping` (`self.CurrentTopping`))))
  (if (`KismetStringLibrary.EqualEqual_StrStr` _returnvalue "Pizza")
    (bind _result (`/Engine/EditorBlueprintResources/StandardMacros.DecrementInt` (`self.AmountPD`))
      (:`  `
        (set `self.AmountPD` _result)))
    (elif (`KismetStringLibrary.EqualEqual_StrStr` _returnvalue "Salami")
      (bind _result_2 (`/Engine/EditorBlueprintResources/StandardMacros.DecrementInt` (`self.AmountSalami`))
        (:`  `
          (set `self.AmountSalami` _result_2)))
      (elif (`KismetStringLibrary.EqualEqual_StrStr` _returnvalue "Paprika")
        (bind _result_3 (`/Engine/EditorBlueprintResources/StandardMacros.DecrementInt` (`self.AmountPaprika`))
          (:`  `
            (set `self.AmountPaprika` _result_3)))))))

(fn `IncreaseToppingsAmount`
  (bind _returnvalue (`|GetEnumeratorNameAsString` (`/Game/Cproef/Blueprints/Cooking/BP_toppings.topping` (`self.CurrentTopping`))))
  (if (`KismetStringLibrary.EqualEqual_StrStr` _returnvalue "Pizza")
    (bind _result (`/Engine/EditorBlueprintResources/StandardMacros.IncrementInt` (`self.AmountPD`))
      (:`  `
        (set `self.AmountPD` _result)))
    (elif (`KismetStringLibrary.EqualEqual_StrStr` _returnvalue "Salami")
      (bind _result_2 (`/Engine/EditorBlueprintResources/StandardMacros.IncrementInt` (`self.AmountSalami`))
        (:`  `
          (set `self.AmountSalami` _result_2)))
      (elif (`KismetStringLibrary.EqualEqual_StrStr` _returnvalue "Paprika")
        (bind _result_3 (`/Engine/EditorBlueprintResources/StandardMacros.IncrementInt` (`self.AmountPaprika`))
          (:`  `
            (set `self.AmountPaprika` _result_3)))))))

(fn `UserConstructionScript`)