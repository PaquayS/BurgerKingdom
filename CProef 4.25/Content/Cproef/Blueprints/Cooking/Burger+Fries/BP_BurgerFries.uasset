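; Burger assembly station for the cooking gameplay: dropped-in ingredient actors build a plated burger in fixed order, from plate and bottom bun up to top bun.
; Each overlap box destroys its matching actor and reveals a pre-hidden mesh, provided the previous layer is visible.
; Buns and meat copy their cook state as a material and deduct from TotalPoints.
; The top bun sets IsFinished, so Tick enables plate physics and moves Scene along with it.
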(event `self.Box6.OnComponentBeginOverlap`
  (params (OverlappedComponent :type "PrimitiveComponent Object Reference") (OtherActor :type "Actor Object Reference") (OtherComp :type "PrimitiveComponent Object Reference") (OtherBodyIndex :type Integer) (bFromSweep :type Boolean) (SweepResult :type "HitResult Structure (by ref)"))
  (bind _plate (`self.Plate`))
  (bind _asbp_burger_plate (cast `/Game/Cproef/Blueprints/Cooking/Burger/BP_BurgerPlate` OtherActor))
  ;[1 1 1] Checking if Cheese is already placed
  (if (not (`SceneComponent.IsVisible` (`self.Plate`)))
    ;[1 1 1] Checking if overlapped Component is Cheese
    (if (== _asbp_burger_plate OtherActor)
      ;[1 1 1] Destroying held burger
      (`self.K2_DestroyActor` OtherActor)
      ;[1 1 1] Setting the correctly placed BMeat visible and collision active
      (`SceneComponent.SetVisibility` _plate true false)
      (`PrimitiveComponent.SetCollisionEnabled` _plate "QueryAndPhysics"))))

(event `self.ReceiveTick`
  (params (DeltaSeconds :type "Float (single-precision)"))
  (bind _plate (`self.Plate`))
  (bind (_returnvalue_x _returnvalue_y _returnvalue_z) (`KismetMathLibrary.BreakVector` (`SceneComponent.K2_GetComponentLocation` _plate)))
  (if (`self.IsFinished?`)
    (`PrimitiveComponent.SetSimulatePhysics` _plate true)
    (`SceneComponent.K2_SetWorldLocation` (`self.Scene`) (`KismetMathLibrary.MakeVector` _returnvalue_x _returnvalue_y (+ _returnvalue_z 1.21)) false false)))

(event `self.Box1.OnComponentBeginOverlap`
  (params (OverlappedComponent :type "PrimitiveComponent Object Reference") (OtherActor :type "Actor Object Reference") (OtherComp :type "PrimitiveComponent Object Reference") (OtherBodyIndex :type Integer) (bFromSweep :type Boolean) (SweepResult :type "HitResult Structure (by ref)"))
  (bind _meat (`self.Meat`))
  (bind _meat_2 (`self.Meat`))
  ;[1 1 1] Putting BurgerMeat check
  (bind _asbp_burger_meat (cast `/Game/Cproef/Blueprints/Cooking/Burger/BP_BurgerMeat` OtherActor))
  ;[1 1 1] checking if bottomBun is already placed
  (if (`SceneComponent.IsVisible` (`self.BBun`))
    ;[1 1 1] Checking if BurgerMeat is already placed
    (if (not (`SceneComponent.IsVisible` (`self.Meat`)))
      ;[1 1 1] Checking if overlapped Component is BMeat
      (if (== OtherActor _asbp_burger_meat)
        ;[1 1 1] Checking how the BMeat is cooked
        (if (`/Game/Cproef/Blueprints/Cooking/Burger/BP_BurgerMeat.IsRaw?` _asbp_burger_meat)
          (set `self.TotalPoints` (- (`self.TotalPoints`) (`self.PointsRaw`)))
          ;[1 1 1] Setting Material
          (`PrimitiveComponent.SetMaterial` _meat 0 "/Game/Cproef/Textures/Testing/M_Uncooked.M_Uncooked")
          ;[1 1 1] Destroying held burger
          (`self.K2_DestroyActor` OtherActor)
          ;[1 1 1] Setting the correctly placed BMeat visible and collision active
          (`SceneComponent.SetVisibility` _meat_2 true false :!label _label)
          (`PrimitiveComponent.SetCollisionEnabled` _meat_2 "QueryAndPhysics")
          (elif (`/Game/Cproef/Blueprints/Cooking/Burger/BP_BurgerMeat.IsCooked?` _asbp_burger_meat)
            (set `self.TotalPoints` (- (`self.TotalPoints`) (`self.PointsCooked`)))
            (`PrimitiveComponent.SetMaterial` _meat 0 "/Game/Cproef/Textures/Testing/M_Cooked.M_Cooked")
            (`self.K2_DestroyActor` OtherActor)
            (goto _label)
            (elif (`/Game/Cproef/Blueprints/Cooking/Burger/BP_BurgerMeat.IsBurned?` _asbp_burger_meat)
              (set `self.TotalPoints` (- (`self.TotalPoints`) (`self.PointsBurned`)))
              (`PrimitiveComponent.SetMaterial` _meat 0 "/Game/Cproef/Textures/Testing/M_Burned.M_Burned")
              (`self.K2_DestroyActor` OtherActor)
              (goto _label))))))))

(event `self.Box.OnComponentBeginOverlap`
  (params (OverlappedComponent :type "PrimitiveComponent Object Reference") (OtherActor :type "Actor Object Reference") (OtherComp :type "PrimitiveComponent Object Reference") (OtherBodyIndex :type Integer) (bFromSweep :type Boolean) (SweepResult :type "HitResult Structure (by ref)"))
  (bind _bbun (`self.BBun`))
  (bind _bbun_2 (`self.BBun`))
  (bind _asbp_bbun (cast `/Game/Cproef/Blueprints/Cooking/Burger/BP_BBun` OtherActor))
  ;[1 1 1] checking if bottomBun is already placed
  (if (`SceneComponent.IsVisible` (`self.Plate`))
    (if (not (`SceneComponent.IsVisible` (`self.BBun`)))
      ;[1 1 1] Checking if overlapped Component is BBun
      (if (== OtherActor _asbp_bbun)
        ;[1 1 1] Checking how the Bun is cooked
        (if (`/Game/Cproef/Blueprints/Cooking/Burger/BP_BBun.IsRaw?` _asbp_bbun)
          (set `self.TotalPoints` (- (`self.TotalPoints`) (`self.PointsRaw`)))
          ;[1 1 1] Setting Material
          (`PrimitiveComponent.SetMaterial` _bbun 0 "/Game/Cproef/Textures/Testing/M_UncookedBun.M_UncookedBun")
          ;[1 1 1] Destroying held burger
          (`self.K2_DestroyActor` OtherActor)
          ;[1 1 1] Setting the correctly placed BMeat visible and collision active
          (`SceneComponent.SetVisibility` _bbun_2 true false :!label _label_2)
          (`PrimitiveComponent.SetCollisionEnabled` _bbun_2 "QueryAndPhysics")
          (elif (`/Game/Cproef/Blueprints/Cooking/Burger/BP_BBun.IsCooked?` _asbp_bbun)
            (set `self.TotalPoints` (- (`self.TotalPoints`) (`self.PointsCooked`)))
            (`PrimitiveComponent.SetMaterial` _bbun 0 "/Game/Cproef/Textures/Testing/M_CookedBun.M_CookedBun")
            (`self.K2_DestroyActor` OtherActor)
            (goto _label_2)
            (elif (`/Game/Cproef/Blueprints/Cooking/Burger/BP_BBun.IsBurned?` _asbp_bbun)
              (set `self.TotalPoints` (- (`self.TotalPoints`) (`self.PointsBurned`)))
              (`PrimitiveComponent.SetMaterial` _bbun 0 "/Game/Cproef/Textures/Testing/M_Burned.M_Burned")
              (`self.K2_DestroyActor` OtherActor)
              (goto _label_2))))))))

(event `self.Box2.OnComponentBeginOverlap`
  (params (OverlappedComponent :type "PrimitiveComponent Object Reference") (OtherActor :type "Actor Object Reference") (OtherComp :type "PrimitiveComponent Object Reference") (OtherBodyIndex :type Integer) (bFromSweep :type Boolean) (SweepResult :type "HitResult Structure (by ref)"))
  (bind _cheese (`self.cheese`))
  ;[1 1 1] Putting cheese check
  (bind _asbp_cheese (cast `/Game/Cproef/Blueprints/Cooking/Burger/BP_Cheese` OtherActor))
  ;[1 1 1] checking if Cheese is already placed
  (if (`SceneComponent.IsVisible` (`self.Meat`))
    ;[1 1 1] Checking if Cheese is already placed
    (if (not (`SceneComponent.IsVisible` (`self.cheese`)))
      ;[1 1 1] Checking if overlapped Component is Cheese
      (if (== _asbp_cheese OtherActor)
        ;[1 1 1] Destroying held burger
        (`self.K2_DestroyActor` OtherActor)
        ;[1 1 1] Setting the correctly placed BMeat visible and collision active
        (`SceneComponent.SetVisibility` _cheese true false)
        (`PrimitiveComponent.SetCollisionEnabled` _cheese "QueryAndPhysics")))))

(event `self.Box3.OnComponentBeginOverlap`
  (params (OverlappedComponent :type "PrimitiveComponent Object Reference") (OtherActor :type "Actor Object Reference") (OtherComp :type "PrimitiveComponent Object Reference") (OtherBodyIndex :type Integer) (bFromSweep :type Boolean) (SweepResult :type "HitResult Structure (by ref)"))
  (bind _onion (`self.onion`))
  (bind _asbp_onion (cast `/Game/Cproef/Blueprints/Cooking/Burger/BP_Onion` OtherActor))
  ;[1 1 1] checking if Cheese is already placed
  (if (`SceneComponent.IsVisible` (`self.cheese`))
    ;[1 1 1] Checking if Cheese is already placed
    (if (not (`SceneComponent.IsVisible` (`self.onion`)))
      ;[1 1 1] Checking if overlapped Component is Cheese
      (if (== _asbp_onion OtherActor)
        ;[1 1 1] Destroying held burger
        (`self.K2_DestroyActor` OtherActor)
        ;[1 1 1] Setting the correctly placed BMeat visible and collision active
        (`SceneComponent.SetVisibility` _onion true false)
        (`PrimitiveComponent.SetCollisionEnabled` _onion "QueryAndPhysics")))))

(event `self.Box4.OnComponentBeginOverlap`
  (params (OverlappedComponent :type "PrimitiveComponent Object Reference") (OtherActor :type "Actor Object Reference") (OtherComp :type "PrimitiveComponent Object Reference") (OtherBodyIndex :type Integer) (bFromSweep :type Boolean) (SweepResult :type "HitResult Structure (by ref)"))
  (bind _tomato (`self.Tomato`))
  (bind _asbp_tomato (cast `/Game/Cproef/Blueprints/Cooking/Burger/BP_Tomato` OtherActor))
  ;[1 1 1] checking if Cheese is already placed
  (if (`SceneComponent.IsVisible` (`self.onion`))
    ;[1 1 1] Checking if Cheese is already placed
    (if (not (`SceneComponent.IsVisible` (`self.Tomato`)))
      ;[1 1 1] Checking if overlapped Component is Cheese
      (if (== _asbp_tomato OtherActor)
        ;[1 1 1] Destroying held burger
        (`self.K2_DestroyActor` OtherActor)
        ;[1 1 1] Setting the correctly placed BMeat visible and collision active
        (`SceneComponent.SetVisibility` _tomato true false)
        (`PrimitiveComponent.SetCollisionEnabled` _tomato "QueryAndPhysics")))))

(event `self.Box5.OnComponentBeginOverlap`
  (params (OverlappedComponent :type "PrimitiveComponent Object Reference") (OtherActor :type "Actor Object Reference") (OtherComp :type "PrimitiveComponent Object Reference") (OtherBodyIndex :type Integer) (bFromSweep :type Boolean) (SweepResult :type "HitResult Structure (by ref)"))
  (bind _tbun (`self.TBun`))
  (bind _tbun_2 (`self.TBun`))
  (bind _asbp_tbun (cast `/Game/Cproef/Blueprints/Cooking/Burger/BP_TBun` OtherActor))
  ;[1 1 1] checking if bottomBun is already placed
  (if (`SceneComponent.IsVisible` (`self.Tomato`))
    ;[1 1 1] Checking if Cheese is already placed
    (if (not (`SceneComponent.IsVisible` (`self.TBun`)))
      ;[1 1 1] Checking if overlapped Component is BBun
      (if (== OtherActor _asbp_tbun)
        ;[1 1 1] Checking how the Bun is cooked
        (if (`/Game/Cproef/Blueprints/Cooking/Burger/BP_TBun.IsRaw?` _asbp_tbun)
          (set `self.TotalPoints` (- (`self.TotalPoints`) (`self.PointsRaw`)))
          ;[1 1 1] Setting Material
          (`PrimitiveComponent.SetMaterial` _tbun 0 "/Game/Cproef/Textures/Testing/M_UncookedBun.M_UncookedBun")
          ;[1 1 1] Destroying held burger
          (`self.K2_DestroyActor` OtherActor)
          ;[1 1 1] Setting the correctly placed BMeat visible and collision active
          (`SceneComponent.SetVisibility` _tbun_2 true false :!label _label_3)
          (`PrimitiveComponent.SetCollisionEnabled` _tbun_2 "QueryAndPhysics")
          (set `self.IsFinished?` true)
          (elif (`/Game/Cproef/Blueprints/Cooking/Burger/BP_TBun.IsCooked?` _asbp_tbun)
            (set `self.TotalPoints` (- (`self.TotalPoints`) (`self.PointsCooked`)))
            (`PrimitiveComponent.SetMaterial` _tbun 0 "/Game/Cproef/Textures/Testing/M_CookedBun.M_CookedBun")
            (`self.K2_DestroyActor` OtherActor)
            (goto _label_3)
            (elif (`/Game/Cproef/Blueprints/Cooking/Burger/BP_TBun.IsBurned?` _asbp_tbun)
              (set `self.TotalPoints` (- (`self.TotalPoints`) (`self.PointsBurned`)))
              (`PrimitiveComponent.SetMaterial` _tbun 0 "/Game/Cproef/Textures/Testing/M_Burned.M_Burned")
              (`self.K2_DestroyActor` OtherActor)
              (goto _label_3))))))))

(fn `UserConstructionScript`
  (bind _bbun (`self.BBun`))
  (bind _meat (`self.Meat`))
  (bind _cheese (`self.cheese`))
  (bind _onion (`self.onion`))
  (bind _tomato (`self.Tomato`))
  (bind _plate (`self.Plate`))
  (bind _tbun (`self.TBun`))
  (`SceneComponent.SetVisibility` _bbun false false)
  (`PrimitiveComponent.SetCollisionEnabled` _bbun "NoCollision")
  (`SceneComponent.SetVisibility` _meat false false)
  (`PrimitiveComponent.SetCollisionEnabled` _meat "NoCollision")
  (`SceneComponent.SetVisibility` _cheese false false)
  (`PrimitiveComponent.SetCollisionEnabled` _cheese "NoCollision")
  (`SceneComponent.SetVisibility` _tomato false false)
  (`PrimitiveComponent.SetCollisionEnabled` _tomato "NoCollision")
  (`SceneComponent.SetVisibility` _onion false false)
  (`PrimitiveComponent.SetCollisionEnabled` _onion "NoCollision")
  (`SceneComponent.SetVisibility` _tbun false false)
  (`PrimitiveComponent.SetCollisionEnabled` _tbun "NoCollision")
  (`SceneComponent.SetVisibility` _plate false false)
  (`PrimitiveComponent.SetCollisionEnabled` _plate "NoCollision"))