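; Grabbable food topping for a cooking game, set up from its Topping enum and ToppingDB row (mesh, materials, thickness, price, starting cook state).
; While IsCooking, Tick advances CookTime through Raw, Cooked and Burned, swapping materials and driving a player-facing progress indicator, hidden for Paprika and Salami.
; BP_MotionController calls Pickup to attach it; Drop detaches it, restoring physics unless AttachedToBurger.
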(event `self.ReceiveTick`
  (params (DeltaSeconds :type "Float (single-precision)"))
  (bind _e (`self.e`))
  (bind _e_2 (`self.e`))
  (bind _cooktime (`self.CookTime`))
  (bind _e_3 (`self.e`))
  (bind _returnvalue (`KismetStringLibrary.Conv_StringToName` (`|GetEnumeratorNameAsString` (`self.topping`))))
  (bind (_returnvalue_roll _returnvalue_pitch _returnvalue_yaw) (`KismetMathLibrary.BreakRotator` (`KismetMathLibrary.FindLookAtRotation` (`SceneComponent.K2_GetComponentLocation` _e_2) (`self.K2_GetActorLocation` (`GameplayStatics.GetPlayerPawn` 0)))))
  (if (`self.IsCooking?`)
    (`self.Cooking`)
    (`self.SetMaterial`)
    (if (== _returnvalue "Paprika")
      (`SceneComponent.SetVisibility` (`self.e`) false false :!label _label)
      (elif (== _returnvalue "Salami")
        (goto _label)
        (else
          (`SceneComponent.SetVisibility` _e_2 true false)
          (`SceneComponent.K2_SetWorldRotation` (`self.e`) (`KismetMathLibrary.MakeRotator` 90.0 0.0 (+ _returnvalue_yaw 270.0)) false false)
          (if (`self.raw?`)
            (`PrimitiveComponent.SetMaterial` _e 0 "/Game/Cproef/Textures/M_CookingR.M_CookingR")
            (`MeshComponent.SetScalarParameterValueOnMaterials` _e_3 "CookTime" (/ _cooktime 15.0))
            (elif (`self.Cooked?`)
              (`PrimitiveComponent.SetMaterial` _e 0 "/Game/Cproef/Textures/M_CookingC.M_CookingC")
              (`MeshComponent.SetScalarParameterValueOnMaterials` _e_3 "CookTime" (/ (- _cooktime 15.0) 15.0))
              (elif (`self.Burned?`)
                (`PrimitiveComponent.SetMaterial` _e 0 "/Game/Cproef/Textures/M_CookingB.M_CookingB")
                (`MeshComponent.SetScalarParameterValueOnMaterials` (`self.e`) "CookTime" (`self.CookTime`))))))))
    (else
      (`SceneComponent.SetVisibility` (`self.e`) false false))))

(event `SetMaterial`
  (bind _staticmeshcomponent (`self.StaticMeshComponent`))
  (bind _staticmeshcomponent_2 (`self.StaticMeshComponent`))
  (bind _staticmeshcomponent_3 (`self.StaticMeshComponent`))
  (bind _returnvalue (`|GetDataTableRow` (`self.ToppingDB`) (`KismetStringLibrary.Conv_StringToName` (`|GetEnumeratorNameAsString` (`self.topping`))))
    (:`then`
      (bind (_matraw1 _mesh _name _size _matc1 _matb1 _toppingthiccness _price _matr2 _matr3 _matc2 _matc3 _matb2 _matb3) (break `/Game/Cproef/Blueprints/Cooking/Struct_Toppings` _returnvalue))
      (`/Engine/EditorBlueprintResources/StandardMacros.IsValid` _matraw1
        (:`Is Valid`
          (if (`self.raw?`)
            (`PrimitiveComponent.SetMaterial` _staticmeshcomponent_3 0 _matraw1)
            (`PrimitiveComponent.SetMaterial` _staticmeshcomponent 0 _matraw1)
            (`PrimitiveComponent.SetMaterial` _staticmeshcomponent 1 _matr2)
            (`PrimitiveComponent.SetMaterial` _staticmeshcomponent 2 _matr3)
            (else
              (`/Engine/EditorBlueprintResources/StandardMacros.IsValid` _matc1
                (:`Is Valid`
                  (if (`self.Cooked?`)
                    (`PrimitiveComponent.SetMaterial` _staticmeshcomponent_3 0 _matc1)
                    (`PrimitiveComponent.SetMaterial` _staticmeshcomponent_3 1 _matc2)
                    (`PrimitiveComponent.SetMaterial` _staticmeshcomponent_3 2 _matc3)
                    (else
                      (`/Engine/EditorBlueprintResources/StandardMacros.IsValid` _matb1
                        (:`Is Valid`
                          (if (`self.Burned?`)
                            (`PrimitiveComponent.SetMaterial` _staticmeshcomponent_3 0 _matb1)
                            (`PrimitiveComponent.SetMaterial` _staticmeshcomponent_2 0 _matb1)
                            (`PrimitiveComponent.SetMaterial` _staticmeshcomponent_2 1 _matb2)
                            (`PrimitiveComponent.SetMaterial` _staticmeshcomponent_2 2 _matb3)
                            (else
                              (`PrimitiveComponent.SetMaterial` _staticmeshcomponent_3 0 null))))))))
                (:`Is Not Valid`
                  (`PrimitiveComponent.SetMaterial` _staticmeshcomponent_3 0 null))))))
        (:`Is Not Valid`
          (`PrimitiveComponent.SetMaterial` _staticmeshcomponent_3 0 null))))))

(event `self.ReceiveBeginPlay`
  (bind _returnvalue (`KismetMathLibrary.RandomFloatInRange` 4.0 6.0))
  (bind _returnvalue_2 (`KismetMathLibrary.RandomFloatInRange` 2.0 4.0))
  (bind _staticmeshcomponent (`self.StaticMeshComponent`))
  (bind _returnvalue_3 (`KismetStringLibrary.Conv_StringToName` (`|GetEnumeratorNameAsString` (`self.topping`))))
  (if (== _returnvalue_3 "Paprika")
    (`SceneComponent.SetWorldScale3D` _staticmeshcomponent (`KismetMathLibrary.MakeVector` _returnvalue_2 _returnvalue_2 _returnvalue_2))
    (elif (== _returnvalue_3 "Salami")
      (`SceneComponent.SetWorldScale3D` _staticmeshcomponent (`KismetMathLibrary.MakeVector` _returnvalue _returnvalue _returnvalue)))))

(event `Cooking`
  (bind _cooktime (`self.CookTime`))
  (set `self.CookTime` (+ (`self.CookTime`) (`GameplayStatics.GetWorldDeltaSeconds`)))
  (if (`KismetMathLibrary.InRange_FloatFloat` _cooktime 0.0 15.0)
    (set `self.raw?` true)
    (set `self.Cooked?` false)
    (set `self.Burned?` false)
    (elif (`KismetMathLibrary.InRange_FloatFloat` _cooktime 15.1 30.0)
      (set `self.raw?` false)
      (set `self.Cooked?` true)
      (set `self.Burned?` false)
      (elif (`KismetMathLibrary.InRange_FloatFloat` _cooktime 30.1 9999999.0)
        (set `self.raw?` false)
        (set `self.Cooked?` false)
        (set `self.Burned?` true)))))

(event `/Game/VirtualRealityBP/Blueprints/PickupActorInterface.Pickup`
  (params (AttachTo :type "SceneComponent Object Reference"))
  (`PrimitiveComponent.SetSimulatePhysics` (`self.StaticMeshComponent`) false)
  (`SceneComponent.K2_AttachToComponent` (`self.K2_GetRootComponent`) AttachTo "None" "KeepWorld" "KeepWorld" "KeepWorld" false))

(event `/Game/VirtualRealityBP/Blueprints/PickupActorInterface.Drop`
  (bind _staticmeshcomponent (`self.StaticMeshComponent`))
  (if (`self.AttachedToBurger?`)
    (`PrimitiveComponent.SetSimulatePhysics` _staticmeshcomponent false)
    (else
      (`PrimitiveComponent.SetSimulatePhysics` _staticmeshcomponent true)))
  (`self.K2_DetachFromActor` "KeepWorld" "KeepWorld" "KeepWorld"))

(fn `UserConstructionScript`
  (bind _staticmeshcomponent (`self.StaticMeshComponent`))
  (bind _staticmeshcomponent_2 (`self.StaticMeshComponent`))
  (bind _returnvalue (`|GetDataTableRow` (`self.ToppingDB`) (`KismetStringLibrary.Conv_StringToName` (`|GetEnumeratorNameAsString` (`self.topping`))))
    (:`then`
      (`|ExecutionSequence`
        (:`then_0`
          (bind (_matraw1 _mesh _name _size _matc1 _matb1 _toppingthiccness _price) (break `/Game/Cproef/Blueprints/Cooking/Struct_Toppings` _returnvalue))
          (`/Engine/EditorBlueprintResources/StandardMacros.IsValid` _mesh
            (:`Is Valid`
              (`StaticMeshComponent.SetStaticMesh` _staticmeshcomponent_2 _mesh)
              (`PrimitiveComponent.SetSimulatePhysics` _staticmeshcomponent_2 true))
            (:`Is Not Valid`
              (`StaticMeshComponent.SetStaticMesh` _staticmeshcomponent_2 null))))
        (:`then_1`
          (`/Engine/EditorBlueprintResources/StandardMacros.IsValid` _matraw1
            (:`Is Valid`
              (`PrimitiveComponent.SetMaterial` _staticmeshcomponent 0 _matraw1))
            (:`Is Not Valid`
              (`PrimitiveComponent.SetMaterial` _staticmeshcomponent 0 null))))
        (:`then_2`
          (bind _returnvalue_2 (`|GetEnumeratorNameAsString` _name))
          ;[1 1 1] Needed to decide if an ingredient is raw or not before spawning it it (buns/meat has to be cooked = raw, other toppings dont need to be cooked = cooked BUT can still be burned so they spawn as ingredients that have already been cooked
          (if (`KismetStringLibrary.EqualEqual_StrStr` _returnvalue_2 "BBuns")
            (set `self.CookTime` 0.0)
            (set `self.raw?` true)
            (set `self.Cooked?` false)
            (set `self.Burned?` false)
            (elif (`KismetStringLibrary.EqualEqual_StrStr` _returnvalue_2 "Meat")
              (set `self.CookTime` 0.0)
              (set `self.raw?` true)
              (set `self.Cooked?` false)
              (set `self.Burned?` false)
              (elif (`KismetStringLibrary.EqualEqual_StrStr` _returnvalue_2 "Cheese")
                (set `self.CookTime` 16.0)
                (set `self.raw?` false)
                (set `self.Cooked?` true)
                (set `self.Burned?` false)
                (elif (`KismetStringLibrary.EqualEqual_StrStr` _returnvalue_2 "Tomato")
                  (set `self.CookTime` 16.0)
                  (set `self.raw?` false)
                  (set `self.Cooked?` true)
                  (set `self.Burned?` false)
                  (elif (`KismetStringLibrary.EqualEqual_StrStr` _returnvalue_2 "Onion")
                    (set `self.CookTime` 16.0)
                    (set `self.raw?` false)
                    (set `self.Cooked?` true)
                    (set `self.Burned?` false)
                    (elif (`KismetStringLibrary.EqualEqual_StrStr` _returnvalue_2 "TBun")
                      (set `self.CookTime` 0.0)
                      (set `self.raw?` true)
                      (set `self.Cooked?` false)
                      (set `self.Burned?` false))))))))
        (:`then_3`
          (set `self.Thiccness` _toppingthiccness))
        (:`then_4`
          (set `self.ToppingPrice` _price))))))