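; BP_PizzaV2 is a pizza that a motion controller can pick up and drop, built by stacking BP_toppings actors and attachable to a plate.
; An overlap detector requires dough first, then snaps each topping on as a non-colliding child.
; Each addition updates topping counts and a cooking score based on raw, cooked or burned state.
; WhatPizza? scores dough plus salami or paprika amounts, while CookingScore and AddToTotalScore are empty.
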(event `self.ReceiveBeginPlay`
  (`SceneComponent.SetWorldScale3D` (`self.StaticMesh`) (2.0 2.0 1.0)))

(event `/Game/VirtualRealityBP/Blueprints/PickupActorInterface.Pickup`
  (params (AttachTo :type "SceneComponent Object Reference"))
  (`PrimitiveComponent.SetSimulatePhysics` (`self.StaticMesh`) false)
  (`SceneComponent.K2_AttachToComponent` (`self.RootComponent`) AttachTo "None" "KeepWorld" "KeepWorld" "KeepWorld" false))

(event `/Game/VirtualRealityBP/Blueprints/PickupActorInterface.Drop`
  (bind _staticmesh (`self.StaticMesh`))
  (if (`self.AttachedToPlate?`)
    (`PrimitiveComponent.SetSimulatePhysics` _staticmesh false)
    (else
      (`PrimitiveComponent.SetSimulatePhysics` _staticmesh true)))
  (`self.K2_DetachFromActor` "KeepWorld" "KeepWorld" "KeepWorld"))

(event `self.ToppingDetector.OnComponentBeginOverlap`
  (params (OverlappedComponent :type "PrimitiveComponent Object Reference") (OtherActor :type "Actor Object Reference") (OtherComp :type "PrimitiveComponent Object Reference") (OtherBodyIndex :type Integer) (bFromSweep :type Boolean) (SweepResult :type "HitResult Structure (by ref)"))
  (bind _currentoffset (`self.CurrentOffset`))
  (bind _currenttopping (`self.CurrentTopping`))
  (bind (_returnvalue_x _returnvalue_y _returnvalue_z) (`KismetMathLibrary.BreakVector` (`SceneComponent.K2_GetComponentLocation` (`self.StaticMesh`))))
  (bind _rootcomponent (`Actor.RootComponent` _currenttopping))
  (bind (_returnvalue_roll _returnvalue_pitch _returnvalue_yaw) (`KismetMathLibrary.BreakRotator` (`SceneComponent.K2_GetComponentRotation` _rootcomponent)))
  (bind (_returnvalue_x_2 _returnvalue_y_2) (`KismetMathLibrary.BreakVector` (`SceneComponent.K2_GetComponentLocation` _rootcomponent)))
  ;[1 1 1] Setting current topping to know what topping you added
  (bind _asbp_toppings (cast `/Game/Cproef/Blueprints/Cooking/BP_toppings` OtherActor))
  (set `self.CurrentTopping` _asbp_toppings)
  (if (== (`self.TotalToppings`) 0)
    (if (== (`KismetStringLibrary.Conv_StringToName` (`|GetEnumeratorNameAsString` (`/Game/Cproef/Blueprints/Cooking/BP_toppings.topping` (`self.CurrentTopping`)))) "Pizza")
      (set `/Game/Cproef/Blueprints/Cooking/BP_toppings.AttachedToBurger?` true _currenttopping :!label _label)
      (`/Game/VirtualRealityBP/Blueprints/PickupActorInterface.Drop` _currenttopping)
      (`PrimitiveComponent.SetCollisionEnabled` (`StaticMeshActor.StaticMeshComponent` _currenttopping) "NoCollision")
      (`self.K2_AttachToActor` _currenttopping self "None" "KeepWorld" "SnapToTarget" "KeepWorld" true)
      (if (== (`KismetStringLibrary.Conv_StringToName` (`|GetEnumeratorNameAsString` (`/Game/Cproef/Blueprints/Cooking/BP_toppings.topping` (`self.CurrentTopping`)))) "Pizza")
        (`SceneComponent.K2_SetRelativeLocation` (`Actor.RootComponent` _currenttopping) (`KismetMathLibrary.MakeVector` 0.0 0.0 (- _currentoffset 0.75)) false true)
        (set `self.CurrentOffset` (+ _currentoffset (`/Game/Cproef/Blueprints/Cooking/BP_toppings.Thiccness` _currenttopping)))
        (else
          (`SceneComponent.K2_SetWorldLocation` _rootcomponent (`KismetMathLibrary.MakeVector` _returnvalue_x_2 _returnvalue_y_2 (+ _currentoffset _returnvalue_z)) false false)
          (`SceneComponent.K2_SetWorldRotation` _rootcomponent (`KismetMathLibrary.MakeRotator` _returnvalue_roll _returnvalue_pitch _returnvalue_yaw) false false)))
      (if (not (`self.RemovingTopping?`))
        (`self.IncreaseToppingsAmount`)
        (`self.AddToTotalScore`)
        (`KismetArrayLibrary.Array_Add` (`self.Toppings`) (`self.CurrentTopping`))
        (`self.CookS`)
        (set `self.CurrentTopping` null)
        (`SceneComponent.K2_SetRelativeLocation` (`self.ToppingDetector`) (0.0 0.0 2.8) false false)
        (set `self.TotalToppings` (+ (`self.TotalToppings`) 1))))
    (else
      (goto _label))))

(event `AttachToPlate`
  (params (PlateToAttachTo :type "/Game/Cproef/Blueprints/Cooking/BP_Plate Object Reference"))
  ;[1 1 1] Attach the food to the plate
  (`self.K2_AttachToActor` PlateToAttachTo "None" "KeepWorld" "KeepWorld" "KeepWorld"))

(event `CookingScore`
  ;[1 1 1] Deciding how good the food has been cooked
)

(event `AddToTotalScore`
  ;[1 1 1] Setting total score of prepared dish
)

(event `WhatPizza?`
  (if (== (`self.AmountDough?`) 1)
    (set `self.TSPizza` (+ (`self.TSPizza`) 2)))
  (if (and (`self.PizzaSal?`) (not (`self.PizzaVeg?`)))
    (if (<= (`self.AmountSalami`) 10)
      (set `self.TSPizza` (+ (`self.TSPizza`) (`self.AmountSalami`)))
      (else
        (set `self.TSPizza` (+ (`self.TSPizza`) (- 10 (`self.AmountSalami`))))))
    (set `self.PizzaSal?` true)
    (elif (and (`self.PizzaVeg?`) (not (`self.PizzaSal?`)))
      (if (<= (`self.AmountPaprika`) 10)
        (set `self.TSPizza` (+ (`self.TSPizza`) (`self.AmountPaprika`)))
        (else
          (set `self.TSPizza` (+ (`self.TSPizza`) (- 10 (`self.AmountPaprika`))))))
      (set `self.PizzaVeg?` true))))

(fn `CookS`
  (if (`/Game/Cproef/Blueprints/Cooking/BP_toppings.raw?` (`self.CurrentTopping`))
    (set `self.CSPizza` (- (`self.CSPizza`) 1))
    (elif (`/Game/Cproef/Blueprints/Cooking/BP_toppings.Cooked?` (`self.CurrentTopping`))
      (set `self.CSPizza` (+ (`self.CSPizza`) 1))
      (elif (`/Game/Cproef/Blueprints/Cooking/BP_toppings.Burned?` (`self.CurrentTopping`))
        (set `self.CSPizza` (+ (`self.CSPizza`) 0))))))

(fn `IncreaseToppingsAmount`
  (bind _returnvalue (`|GetEnumeratorNameAsString` (`/Game/Cproef/Blueprints/Cooking/BP_toppings.topping` (`self.CurrentTopping`))))
  (if (`KismetStringLibrary.EqualEqual_StrStr` _returnvalue "Pizza")
    (bind _result (`/Engine/EditorBlueprintResources/StandardMacros.IncrementInt` (`self.AmountDough?`))
      (:`  `
        (set `self.AmountDough?` _result)))
    (elif (`KismetStringLibrary.EqualEqual_StrStr` _returnvalue "Salami")
      (bind _result_2 (`/Engine/EditorBlueprintResources/StandardMacros.IncrementInt` (`self.AmountSalami`))
        (:`  `
          (set `self.AmountSalami` _result_2)))
      (elif (`KismetStringLibrary.EqualEqual_StrStr` _returnvalue "Paprika")
        (bind _result_3 (`/Engine/EditorBlueprintResources/StandardMacros.IncrementInt` (`self.AmountPaprika`))
          (:`  `
            (set `self.AmountPaprika` _result_3)))))))

(fn `UserConstructionScript`)