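; Stackable VR burger that BP_MotionController picks up and that can be attached to a plate.
; An overlap detector requires a bottom bun first, then snaps each BP_toppings on at a rising height offset.
; Each addition updates per-type counts and a cooking score, while WhatBurger tallies topping score and flags burger or cheeseburger.
; The older ScoreTot scoring events are empty stubs, with their logic left unconnected.
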(event `/Game/VirtualRealityBP/Blueprints/PickupActorInterface.Pickup`
  (params (AttachTo :type "SceneComponent Object Reference"))
  (`PrimitiveComponent.SetSimulatePhysics` (`self.StaticMesh`) false)
  (`SceneComponent.K2_AttachToComponent` (`self.RootComponent`) AttachTo "None" "KeepWorld" "KeepWorld" "KeepWorld" false))

(event `/Game/VirtualRealityBP/Blueprints/PickupActorInterface.Drop`
  (bind _staticmesh (`self.StaticMesh`))
  (if (`self.AttachedToPlate?`)
    (`PrimitiveComponent.SetSimulatePhysics` _staticmesh false)
    (else
      (`PrimitiveComponent.SetSimulatePhysics` _staticmesh true)))
  (`self.K2_DetachFromActor` "KeepWorld" "KeepWorld" "KeepWorld"))

(event `self.ToppingDetector.OnComponentBeginOverlap`
  (params (OverlappedComponent :type "PrimitiveComponent Object Reference") (OtherActor :type "Actor Object Reference") (OtherComp :type "PrimitiveComponent Object Reference") (OtherBodyIndex :type Integer) (bFromSweep :type Boolean) (SweepResult :type "HitResult Structure (by ref)"))
  (bind _currentoffset (`self.CurrentOffset`))
  (bind _currenttopping (`self.CurrentTopping`))
  ;[1 1 1] Setting current topping to know what topping you added
  (bind _asbp_toppings (cast `/Game/Cproef/Blueprints/Cooking/BP_toppings` OtherActor))
  (set `self.CurrentTopping` _asbp_toppings)
  (if (`self.BottomBunPlaced?`)
    (`/Engine/EditorBlueprintResources/StandardMacros.IsValid` _currenttopping :!label _label
      (:`Is Valid`
        (set `/Game/Cproef/Blueprints/Cooking/BP_toppings.AttachedToBurger?` true _currenttopping)
        (`/Game/VirtualRealityBP/Blueprints/PickupActorInterface.Drop` _currenttopping)
        (`PrimitiveComponent.SetCollisionEnabled` (`StaticMeshActor.StaticMeshComponent` _currenttopping) "NoCollision")
        (`self.K2_AttachToActor` _currenttopping self "None" "SnapToTarget" "SnapToTarget" "KeepWorld" true)
        (`SceneComponent.K2_SetRelativeLocation` (`Actor.RootComponent` _currenttopping) (`KismetMathLibrary.MakeVector` 0.0 0.0 (- _currentoffset 0.75)) false true)
        (bind _output_get (set `self.CurrentOffset` (+ _currentoffset (`/Game/Cproef/Blueprints/Cooking/BP_toppings.Thiccness` _currenttopping))))
        (if (not (`self.RemovingTopping?`))
          (`self.IncreaseToppingsAmount`)
          (`self.AddToTotalScore`)
          (`KismetArrayLibrary.Array_Add` (`self.Toppings`) (`self.CurrentTopping`))
          (`self.CookS`)
          (set `self.CurrentTopping` null)
          (`SceneComponent.K2_SetRelativeLocation` (`self.ToppingDetector`) (`KismetMathLibrary.MakeVector` 0.0 0.0 _output_get) false false)
          (set `self.BottomBunPlaced?` true))))
    (elif (== (`KismetStringLibrary.Conv_StringToName` (`|GetEnumeratorNameAsString` (`/Game/Cproef/Blueprints/Cooking/BP_toppings.topping` (`self.CurrentTopping`)))) "BBuns")
      (goto _label))))

(event `AttachToPlate`
  (params (PlateToAttachTo :type "/Game/Cproef/Blueprints/Cooking/BP_Plate Object Reference"))
  ;[1 1 1] Attach the food to the plate
  (`self.K2_AttachToActor` PlateToAttachTo "None" "KeepWorld" "KeepWorld" "KeepWorld")
  (`self.ToppingScore`)
  (set `self.ScoreTot` (+ (`self.ScoreTop`) (`self.ScoreTot`))))

(event `CookingScore`
  ;[1 1 1] Deciding how good the food has been cooked
)

(event `RemoveFromTotalScore`)

(event `AddToTotalScore`
  ;[1 1 1] Setting total score of prepared dish
)

(event `ToppingScore`)

(event `self.ReceiveBeginPlay`)

(event `WhatBurger`
  (if (== (`self.AmountBBuns`) 1)
    (`self.TopS`))
  (if (== (`self.AmountMeat`) 1)
    (`self.TopS`))
  (if (== (`self.AmountTBuns`) 1)
    (`self.TopS`))
  (if (== (`self.AmountOnions`) 1)
    (`self.TopS`))
  (if (== (`self.AmountTomatoes`) 1)
    (`self.TopS`))
  (if (== (`self.AmountCheese`) 1)
    (set `self.CheeseBurger?` true :!label _label_2)
    (elif (== (`self.AmountCheese`) 0)
      (set `self.Burger?` true)
      (else
        (goto _label_2)))))

(event `CookingGrade?`)

(fn `CookS`
  (if (`/Game/Cproef/Blueprints/Cooking/BP_toppings.raw?` (`self.CurrentTopping`))
    (set `self.CS` (- (`self.CS`) 1))
    (elif (`/Game/Cproef/Blueprints/Cooking/BP_toppings.Cooked?` (`self.CurrentTopping`))
      (set `self.CS` (+ (`self.CS`) 2))
      (elif (`/Game/Cproef/Blueprints/Cooking/BP_toppings.Burned?` (`self.CurrentTopping`))
        (set `self.CS` (+ (`self.CS`) 0))))))

(fn `DecreaseToppingsAmount`
  (bind _returnvalue (`|GetEnumeratorNameAsString` (`/Game/Cproef/Blueprints/Cooking/BP_toppings.topping` (`self.CurrentTopping`))))
  (if (`KismetStringLibrary.EqualEqual_StrStr` _returnvalue "BBun")
    (bind _result (`/Engine/EditorBlueprintResources/StandardMacros.DecrementInt` (`self.AmountBBuns`))
      (:`  `
        (set `self.AmountBBuns` _result)))
    (elif (`KismetStringLibrary.EqualEqual_StrStr` _returnvalue "Meat")
      (bind _result_2 (`/Engine/EditorBlueprintResources/StandardMacros.DecrementInt` (`self.AmountMeat`))
        (:`  `
          (set `self.AmountMeat` _result_2)))
      (elif (`KismetStringLibrary.EqualEqual_StrStr` _returnvalue "Cheese")
        (bind _result_3 (`/Engine/EditorBlueprintResources/StandardMacros.DecrementInt` (`self.AmountCheese`))
          (:`  `
            (set `self.AmountCheese` _result_3)))
        (elif (`KismetStringLibrary.EqualEqual_StrStr` _returnvalue "Tomato")
          (bind _result_4 (`/Engine/EditorBlueprintResources/StandardMacros.DecrementInt` (`self.AmountTomatoes`))
            (:`  `
              (set `self.AmountTomatoes` _result_4)))
          (elif (`KismetStringLibrary.EqualEqual_StrStr` _returnvalue "Onion")
            (bind _result_5 (`/Engine/EditorBlueprintResources/StandardMacros.DecrementInt` (`self.AmountOnions`))
              (:`  `
                (set `self.AmountOnions` _result_5)))
            (elif (`KismetStringLibrary.EqualEqual_StrStr` _returnvalue "TBun")
              (bind _result_6 (`/Engine/EditorBlueprintResources/StandardMacros.DecrementInt` (`self.AmountTBuns`))
                (:`  `
                  (set `self.AmountTBuns` _result_6))))))))))

(fn `IncreaseToppingsAmount`
  (bind _returnvalue (`|GetEnumeratorNameAsString` (`/Game/Cproef/Blueprints/Cooking/BP_toppings.topping` (`self.CurrentTopping`))))
  (if (`KismetStringLibrary.EqualEqual_StrStr` _returnvalue "BBuns")
    (bind _result (`/Engine/EditorBlueprintResources/StandardMacros.IncrementInt` (`self.AmountBBuns`))
      (:`  `
        (set `self.AmountBBuns` _result)))
    (elif (`KismetStringLibrary.EqualEqual_StrStr` _returnvalue "Meat")
      (bind _result_2 (`/Engine/EditorBlueprintResources/StandardMacros.IncrementInt` (`self.AmountMeat`))
        (:`  `
          (set `self.AmountMeat` _result_2)))
      (elif (`KismetStringLibrary.EqualEqual_StrStr` _returnvalue "Cheese")
        (bind _result_3 (`/Engine/EditorBlueprintResources/StandardMacros.IncrementInt` (`self.AmountCheese`))
          (:`  `
            (set `self.AmountCheese` _result_3)))
        (elif (`KismetStringLibrary.EqualEqual_StrStr` _returnvalue "Tomato")
          (bind _result_4 (`/Engine/EditorBlueprintResources/StandardMacros.IncrementInt` (`self.AmountTomatoes`))
            (:`  `
              (set `self.AmountTomatoes` _result_4)))
          (elif (`KismetStringLibrary.EqualEqual_StrStr` _returnvalue "Onion")
            (bind _result_5 (`/Engine/EditorBlueprintResources/StandardMacros.IncrementInt` (`self.AmountOnions`))
              (:`  `
                (set `self.AmountOnions` _result_5)))
            (elif (`KismetStringLibrary.EqualEqual_StrStr` _returnvalue "TBun")
              (bind _result_6 (`/Engine/EditorBlueprintResources/StandardMacros.IncrementInt` (`self.AmountTBuns`))
                (:`  `
                  (set `self.AmountTBuns` _result_6))))))))))

(fn `TopS`
  (set `self.TS` (+ (`self.TS`) 1)))

(fn `UserConstructionScript`)