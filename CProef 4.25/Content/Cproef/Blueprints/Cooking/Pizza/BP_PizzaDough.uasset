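; BP_PizzaDough is a cookable pizza dough actor that tracks whether it is raw, cooked or burned.
; While IsCooking is set, Tick accumulates delta seconds into CookTime, prints it, and compares it against fixed time ranges.
; Each range sets the doneness flags and swaps the BBun mesh's material to match.
; A separate IncrementT function bumps and prints CookTime but is not called within this graph.
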(event `self.ReceiveBeginPlay`)

(event `self.ReceiveTick`
  (params (DeltaSeconds :type "Float (single-precision)"))
  (bind _bbun (`self.BBun`))
  (bind _cooktime (`self.CookTime`))
  ;[1 1 1] Checking if cooking
  (if (`self.IsCooking?`)
    ;[1 1 1] Checking duration of cooking
    (bind _output_get (set `self.CookTime` (+ _cooktime (`GameplayStatics.GetWorldDeltaSeconds`))))
    (`KismetSystemLibrary.PrintString` (`KismetStringLibrary.Conv_DoubleToString` _output_get))
    (if (`KismetMathLibrary.InRange_FloatFloat` _cooktime 0.0 15.0)
      ;[1 1 1] Affects customer happiness/setting cooked status
      (set `self.IsRaw?` true)
      (set `self.IsCooked?` false)
      (set `self.IsBurned?` false)
      ;[1 1 1] Changing materials based on cooked
      (`PrimitiveComponent.SetMaterial` _bbun 0 "/Game/Cproef/Textures/Testing/M_UncookedBun.M_UncookedBun")
      (elif (`KismetMathLibrary.InRange_FloatFloat` _cooktime 15.1 30.0)
        (set `self.IsCooked?` true)
        (set `self.IsRaw?` false)
        (set `self.IsBurned?` false)
        (`PrimitiveComponent.SetMaterial` _bbun 0 "/Game/Cproef/Textures/Testing/M_CookedBun.M_CookedBun")
        (elif (`KismetMathLibrary.InRange_FloatFloat` _cooktime 30.1 9999999.0)
          (set `self.IsBurned?` true)
          (set `self.IsRaw?` false)
          (set `self.IsCooked?` false)
          (`PrimitiveComponent.SetMaterial` _bbun 0 "/Game/Cproef/Textures/Testing/M_Burned.M_Burned"))))))

(fn `IncrementT`
  (bind _output_get (set `self.CookTime` (+ (`self.CookTime`) 1.0)))
  (`KismetSystemLibrary.PrintString` (`KismetStringLibrary.Conv_DoubleToString` _output_get)))

(fn `UserConstructionScript`)