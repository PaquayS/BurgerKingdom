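; BP_PizzaCooker is a cooking zone that cooks the toppings of any BP_PizzaV2 inside its box trigger.
; Box overlap begin and end toggle IsCooking on each of the pizza's toppings, leaving any cooking logic outside this Blueprint.
; The same topping loops start and stop the cooking audio, so a pizza without toppings leaves the sound unchanged.
; Audio is also stopped on BeginPlay.
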(event `self.ReceiveBeginPlay`
  (`AudioComponent.Stop` (`self.Audio`)))

(event `self.Box.OnComponentBeginOverlap`
  (params (OverlappedComponent :type "PrimitiveComponent Object Reference") (OtherActor :type "Actor Object Reference") (OtherComp :type "PrimitiveComponent Object Reference") (OtherBodyIndex :type Integer) (bFromSweep :type Boolean) (SweepResult :type "HitResult Structure (by ref)"))
  (bind _asbp_pizza_v2 (cast `/Game/Cproef/Blueprints/Cooking/BP_PizzaV2` OtherActor))
  (for _array_element (`/Game/Cproef/Blueprints/Cooking/BP_PizzaV2.Toppings` _asbp_pizza_v2)
    (set `/Game/Cproef/Blueprints/Cooking/BP_toppings.IsCooking?` true _array_element)
    (set `self.PlayAudio?` true)
    (`AudioComponent.Play` (`self.Audio`) 0.0)))

(event `self.Box.OnComponentEndOverlap`
  (params (OverlappedComponent :type "PrimitiveComponent Object Reference") (OtherActor :type "Actor Object Reference") (OtherComp :type "PrimitiveComponent Object Reference") (OtherBodyIndex :type Integer))
  (bind _asbp_pizza_v2 (cast `/Game/Cproef/Blueprints/Cooking/BP_PizzaV2` OtherActor))
  (for _array_element (`/Game/Cproef/Blueprints/Cooking/BP_PizzaV2.Toppings` _asbp_pizza_v2)
    (set `/Game/Cproef/Blueprints/Cooking/BP_toppings.IsCooking?` false _array_element)
    (set `self.PlayAudio?` false)
    (`AudioComponent.Stop` (`self.Audio`))))

(fn `UserConstructionScript`)