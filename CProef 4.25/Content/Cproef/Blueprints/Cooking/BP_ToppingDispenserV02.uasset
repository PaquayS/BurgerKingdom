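; VR cooking dispenser that sells the topping selected by ToppingName.
; Overlap of its Button by a motion controller or StaticMeshActor spawns a BP_toppings at SpawnLocation and deducts the ToppingDB price from the MotionControllerPawn's Wallet.
; The construction script sets the display mesh and materials from the same table, giving Paprika and Salami raw materials and a larger scale.
; A Tick-played timeline drives the yaw of RotatePoint.
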(event `SpawnTopping`
  (bind _toppingname (`self.ToppingName`))
  (bind _returnvalue_location (`KismetMathLibrary.BreakTransform` (`SceneComponent.K2_GetComponentToWorld` (`self.SpawnLocation`))))
  (`|SpawnActorFromClass` "/Game/Cproef/Blueprints/Cooking/BP_toppings.BP_toppings_C" (`KismetMathLibrary.MakeTransform` _returnvalue_location) "Undefined" "OverrideRootScale" null _toppingname null)
  (bind _returnvalue (`|GetDataTableRow` (`self.ToppingDB`) (`KismetStringLibrary.Conv_StringToName` (`|GetEnumeratorNameAsString` _toppingname)))
    (:`then`
      (bind _returnvalue_2 (`GameplayStatics.GetActorOfClass` "/Game/VirtualRealityBP/Blueprints/MotionControllerPawn.MotionControllerPawn_C"))
      (set `/Game/VirtualRealityBP/Blueprints/MotionControllerPawn.Wallet` (- (`/Game/VirtualRealityBP/Blueprints/MotionControllerPawn.Wallet` _returnvalue_2) (`.Price_28_D6C3A49C4A2A7DFBC700F099CF0EA2A6` (break `/Game/Cproef/Blueprints/Cooking/Struct_Toppings` _returnvalue))) _returnvalue_2))))

(event `self.Button.OnComponentBeginOverlap`
  (params (OverlappedComponent :type "PrimitiveComponent Object Reference") (OtherActor :type "Actor Object Reference") (OtherComp :type "PrimitiveComponent Object Reference") (OtherBodyIndex :type Integer) (bFromSweep :type Boolean) (SweepResult :type "HitResult Structure (by ref)"))
  (bind _returnvalue (`GameplayStatics.GetObjectClass` OtherActor))
  (if (== _returnvalue "/Script/Engine.StaticMeshActor")
    (`self.SpawnTopping` :!label _label)
    (elif (== _returnvalue "/Game/VirtualRealityBP/Blueprints/BP_MotionController.BP_MotionController_C")
      (goto _label))))

(event `self.ReceiveTick`
  (params (DeltaSeconds :type "Float (single-precision)"))
  (bind (_direction _newtrack_0) (`Timeline|Timeline_0`)
    (:`Update`
      (`SceneComponent.K2_SetRelativeRotation` (`self.RotatePoint`) (`KismetMathLibrary.MakeRotator` 0.0 0.0 _newtrack_0) false false))))

(fn `UserConstructionScript`
  (bind _staticmesh (`self.StaticMesh`))
  (bind _staticmesh_2 (`self.StaticMesh`))
  (bind _returnvalue (`KismetStringLibrary.Conv_StringToName` (`|GetEnumeratorNameAsString` (`self.ToppingName`))))
  (if (== _returnvalue "Paprika")
    (bind _returnvalue_2 (`|GetDataTableRow` (`self.ToppingDB`) _returnvalue :!label _label)
      (:`then`
        (bind (_matraw1 _mesh _name _size _matc1 _matb1 _toppingthiccness _price _matr2 _matr3) (break `/Game/Cproef/Blueprints/Cooking/Struct_Toppings` _returnvalue_2))
        (`StaticMeshComponent.SetStaticMesh` (`self.StaticMesh`) _mesh)
        (`PrimitiveComponent.SetMaterial` _staticmesh_2 0 _matraw1)
        (`PrimitiveComponent.SetMaterial` _staticmesh_2 1 _matr2)
        (`PrimitiveComponent.SetMaterial` _staticmesh_2 2 _matr3)
        (`SceneComponent.SetWorldScale3D` (`self.StaticMesh`) (2.0 2.0 2.0))))
    (elif (== _returnvalue "Salami")
      (goto _label)
      (else
        (bind _returnvalue_3 (`|GetDataTableRow` (`self.ToppingDB`) _returnvalue)
          (:`then`
            (bind (_matraw1_2 _mesh_2 _name_2 _size_2 _matc1_2 _matb1_2 _toppingthiccness_2 _price_2 _matr2_2 _matr3_2 _matc2 _matc3) (break `/Game/Cproef/Blueprints/Cooking/Struct_Toppings` _returnvalue_3))
            (`StaticMeshComponent.SetStaticMesh` (`self.StaticMesh`) _mesh_2)
            (`PrimitiveComponent.SetMaterial` _staticmesh 0 _matc1_2)
            (`PrimitiveComponent.SetMaterial` _staticmesh 1 _matc2)
            (`PrimitiveComponent.SetMaterial` _staticmesh 2 _matc3)))))))