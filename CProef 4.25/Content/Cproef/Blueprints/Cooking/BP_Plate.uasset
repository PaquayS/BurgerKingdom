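; BP_Plate is a serving plate for a cooking game, picked up and dropped through BP_MotionController.
; Its Box overlap snaps a burger or pizza to the Scene point without collision, then records TotalScore and dish-type flags.
; AttachToAI snaps the plate to a parent component and calls AcceptedOrder on the owning BP_AIChar01.
; Dish removal and tip logic is disconnected, and the graphs never call VelocityCalculation.
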(event `/Game/VirtualRealityBP/Blueprints/PickupActorInterface.Pickup`
  (params (AttachTo :type "SceneComponent Object Reference"))
  (`PrimitiveComponent.SetSimulatePhysics` (`self.StaticMeshComponent`) false)
  (`SceneComponent.K2_AttachToComponent` (`self.K2_GetRootComponent`) AttachTo "None" "KeepWorld" "KeepWorld" "KeepWorld" false))

(event `/Game/VirtualRealityBP/Blueprints/PickupActorInterface.Drop`
  (`PrimitiveComponent.SetSimulatePhysics` (`self.StaticMeshComponent`) true)
  (`self.K2_DetachFromActor` "KeepWorld" "KeepWorld" "KeepWorld"))

(event `self.ReceiveTick`
  (params (DeltaSeconds :type "Float (single-precision)")))

(event `self.Box.OnComponentBeginOverlap`
  (params (OverlappedComponent :type "PrimitiveComponent Object Reference") (OtherActor :type "Actor Object Reference") (OtherComp :type "PrimitiveComponent Object Reference") (OtherBodyIndex :type Integer) (bFromSweep :type Boolean) (SweepResult :type "HitResult Structure (by ref)"))
  (bind _pizza (`self.Pizza`))
  (bind _food (`self.Food`))
  (bind _food_2 (`self.Food`))
  (bind _food_3 (`self.Food`))
  (bind _pizza_2 (`self.Pizza`))
  (bind _pizza_3 (`self.Pizza`))
  (bind _asbp_burger_v2 (cast `/Game/Cproef/Blueprints/Cooking/BP_BurgerV2` OtherActor)
    (:`then`
      (set `self.Food` _asbp_burger_v2)
      (`/Engine/EditorBlueprintResources/StandardMacros.IsValid` _food
        (:`Is Valid`
          (set `/Game/Cproef/Blueprints/Cooking/BP_BurgerV2.AttachedToPlate?` true _asbp_burger_v2)
          (`/Game/VirtualRealityBP/Blueprints/PickupActorInterface.Drop` _food)
          (`PrimitiveComponent.SetCollisionEnabled` (`/Game/Cproef/Blueprints/Cooking/BP_BurgerV2.StaticMesh` _food) "NoCollision")
          (`self.K2_AttachToActor` _food self "None" "KeepWorld" "KeepWorld" "KeepWorld" true)
          (`SceneComponent.K2_SetRelativeLocation` (`Actor.RootComponent` _food) (`SceneComponent.RelativeLocation` (`self.Scene`)) false false)
          (`/Game/Cproef/Blueprints/Cooking/BP_BurgerV2.WhatBurger` _food_3)
          (set `self.TotalScore` (+ (`/Game/Cproef/Blueprints/Cooking/BP_BurgerV2.CS` _food_3) (`/Game/Cproef/Blueprints/Cooking/BP_BurgerV2.TS` _food_3)))
          (if (`/Game/Cproef/Blueprints/Cooking/BP_BurgerV2.CheeseBurger?` _food_2)
            (set `self.CB?` true)
            (elif (`/Game/Cproef/Blueprints/Cooking/BP_BurgerV2.Burger?` _food_2)
              (set `self.B?` true))))))
    (:`CastFailed`
      (bind _asbp_pizza_v2 (cast `/Game/Cproef/Blueprints/Cooking/BP_PizzaV2` OtherActor)
        (:`then`
          (set `self.Pizza` _asbp_pizza_v2)
          (`/Engine/EditorBlueprintResources/StandardMacros.IsValid` _pizza
            (:`Is Valid`
              (set `/Game/Cproef/Blueprints/Cooking/BP_PizzaV2.AttachedToPlate?` false _asbp_pizza_v2)
              (`/Game/VirtualRealityBP/Blueprints/PickupActorInterface.Drop` _pizza)
              (`PrimitiveComponent.SetCollisionEnabled` (`/Game/Cproef/Blueprints/Cooking/BP_PizzaV2.StaticMesh` _pizza) "NoCollision")
              (`self.K2_AttachToActor` _pizza self "None" "KeepWorld" "KeepWorld" "KeepWorld" true)
              (`SceneComponent.K2_SetRelativeLocation` (`Actor.RootComponent` _pizza) (`SceneComponent.RelativeLocation` (`self.Scene`)) false false)
              (`/Game/Cproef/Blueprints/Cooking/BP_PizzaV2.WhatPizza?` _pizza_2)
              (set `self.TotalScore` (+ (`/Game/Cproef/Blueprints/Cooking/BP_PizzaV2.CSPizza` _pizza_2) (`/Game/Cproef/Blueprints/Cooking/BP_PizzaV2.TSPizza` _pizza_2)))
              (if (`/Game/Cproef/Blueprints/Cooking/BP_PizzaV2.PizzaVeg?` _pizza_3)
                (set `self.PV?` true)
                (elif (`/Game/Cproef/Blueprints/Cooking/BP_PizzaV2.PizzaSal?` _pizza_3)
                  (set `self.PS?` true))))))
        (:`CastFailed`
          (bind _asbp_motion_controller (cast `/Game/VirtualRealityBP/Blueprints/BP_MotionController` OtherActor))
          (set `self.DetectedMotionController` _asbp_motion_controller))))))

(event `self.Box.OnComponentEndOverlap`
  (params (OverlappedComponent :type "PrimitiveComponent Object Reference") (OtherActor :type "Actor Object Reference") (OtherComp :type "PrimitiveComponent Object Reference") (OtherBodyIndex :type Integer)))

(fn `AttachToAI`
  (params (AttachTOParent :type "SceneComponent Object Reference"))
  (bind _staticmeshcomponent (`self.StaticMeshComponent`))
  (`PrimitiveComponent.SetSimulatePhysics` _staticmeshcomponent false)
  (`PrimitiveComponent.SetCollisionResponseToChannel` _staticmeshcomponent "ECC_Pawn" "ECR_Ignore")
  (`self.K2_AttachToComponent` AttachTOParent "None" "SnapToTarget" "SnapToTarget" "KeepRelative")
  (bind _asbp_aichar_01 (cast `/Game/Cproef/test/BP_AIChar01` (`ActorComponent.GetOwner` AttachTOParent)))
  (`/Game/Cproef/test/BP_AIChar01.AcceptedOrder` _asbp_aichar_01))

(fn `UserConstructionScript`)

(fn `VelocityCalculation`
  (params (CurrentPosition :type "Vector Structure") (DeltaSeconds :type "Float (double-precision)"))
  (bind _output_get (set `self.CurrentTime` (+ (`self.PreviousTime`) DeltaSeconds)))
  (set `self.CurrentPosition` CurrentPosition)
  (set `self.Velocity` (`KismetMathLibrary.VSize` (/ (- (`self.CurrentPosition`) (`self.PreviousPosition`)) (- _output_get (`self.PreviousTime`)))))
  (set `self.PreviousTime` (`self.CurrentTime`))
  (set `self.PreviousPosition` (`self.CurrentPosition`)))