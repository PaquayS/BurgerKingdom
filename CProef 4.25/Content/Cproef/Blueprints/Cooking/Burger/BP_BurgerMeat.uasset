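; BP_BurgerMeat is a burger patty for the cooking gameplay that turns from raw to cooked to burned.
; While IsCooking is set, Tick accumulates CookTime and uses range checks to set the exclusive doneness flags and swap the Meat material.
; A note marks the raw state as affecting customer happiness, though that logic is not here.
; IncrementT adds a fixed step to CookTime, and an older flag-driven material chain is left unconnected.
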(event `self.ReceiveBeginPlay`)

(event `self.ReceiveTick`
  (params (DeltaSeconds :type "Float (single-precision)"))
  (bind _meat (`self.Meat`))
  (bind _cooktime (`self.CookTime`))
  (if (`self.IsCooking?`)
    (set `self.CookTime` (+ _cooktime (`GameplayStatics.GetWorldDeltaSeconds`)))
    (if (`KismetMathLibrary.InRange_FloatFloat` _cooktime 0.0 15.0)
      ;[1 1 1] Affects customer happiness
      (set `self.IsRaw?` true)
      (set `self.IsCooked?` false)
      (set `self.IsBurned?` false)
      (`PrimitiveComponent.SetMaterial` _meat 0 "/Game/Cproef/Textures/Testing/M_Uncooked.M_Uncooked")
      (elif (`KismetMathLibrary.InRange_FloatFloat` _cooktime 15.1 30.0)
        (set `self.IsCooked?` true)
        (set `self.IsRaw?` false)
        (set `self.IsBurned?` false)
        (`PrimitiveComponent.SetMaterial` _meat 0 "/Game/Cproef/Textures/Testing/M_Cooked.M_Cooked")
        (elif (`KismetMathLibrary.InRange_FloatFloat` _cooktime 30.1 9999999.0)
          (set `self.IsBurned?` true)
          (set `self.IsRaw?` false)
          (set `self.IsCooked?` false)
          (`PrimitiveComponent.SetMaterial` _meat 0 "/Game/Cproef/Textures/Testing/M_Burned.M_Burned"))))))

(fn `IncrementT`
  (set `self.CookTime` (+ (`self.CookTime`) 1.0)))

(fn `UserConstructionScript`)