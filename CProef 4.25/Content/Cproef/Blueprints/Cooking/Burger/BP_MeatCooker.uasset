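; BP_MeatCooker is a cooking surface for the burger station that marks toppings as cooking while they are on it.
; Its Box trigger sets IsCooking on each overlapping BP_toppings and clears it when that topping leaves.
; Audio is silenced at BeginPlay, restarts whenever a topping enters and stops when any topping exits, even if others remain inside.
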(event `self.ReceiveBeginPlay`
  (`AudioComponent.Stop` (`self.Audio`)))

(event `self.Box.OnComponentBeginOverlap`
  (params (OverlappedComponent :type "PrimitiveComponent Object Reference") (OtherActor :type "Actor Object Reference") (OtherComp :type "PrimitiveComponent Object Reference") (OtherBodyIndex :type Integer) (bFromSweep :type Boolean) (SweepResult :type "HitResult Structure (by ref)"))
  (bind _asbp_toppings (cast `/Game/Cproef/Blueprints/Cooking/BP_toppings` OtherActor))
  (set `/Game/Cproef/Blueprints/Cooking/BP_toppings.IsCooking?` true _asbp_toppings)
  (`AudioComponent.Play` (`self.Audio`) 0.0))

(event `self.Box.OnComponentEndOverlap`
  (params (OverlappedComponent :type "PrimitiveComponent Object Reference") (OtherActor :type "Actor Object Reference") (OtherComp :type "PrimitiveComponent Object Reference") (OtherBodyIndex :type Integer))
  (bind _asbp_toppings (cast `/Game/Cproef/Blueprints/Cooking/BP_toppings` OtherActor))
  (set `/Game/Cproef/Blueprints/Cooking/BP_toppings.IsCooking?` false _asbp_toppings)
  (`AudioComponent.Stop` (`self.Audio`)))

(fn `UserConstructionScript`)