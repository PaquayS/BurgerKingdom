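; BP_Burger1 is a burger assembly actor on a plate that scores how well its ingredients are cooked.
; Only the bottom bun overlap is live: it deducts points for the raw, cooked or burned state, then calls AttachToPlate to snap-attach at BBunLoc with plate physics off.
; Other overlap events are empty.
; Disconnected logic remains for further ingredients, revealing hidden placed meshes and destroying held actors, plus finished-plate physics.
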(event `self.ReceiveTick`
  (params (DeltaSeconds :type "Float (single-precision)")))

(event `self.Box1.OnComponentBeginOverlap`
  (params (OverlappedComponent :type "PrimitiveComponent Object Reference") (OtherActor :type "Actor Object Reference") (OtherComp :type "PrimitiveComponent Object Reference") (OtherBodyIndex :type Integer) (bFromSweep :type Boolean) (SweepResult :type "HitResult Structure (by ref)"))
  ;[1 1 1] Putting BurgerMeat check
)

(event `self.Box.OnComponentBeginOverlap`
  (params (OverlappedComponent :type "PrimitiveComponent Object Reference") (OtherActor :type "Actor Object Reference") (OtherComp :type "PrimitiveComponent Object Reference") (OtherBodyIndex :type Integer) (bFromSweep :type Boolean) (SweepResult :type "HitResult Structure (by ref)"))
  (if (not (`self.BBun?`))
    (bind _asbp_bbun (cast `/Game/Cproef/Blueprints/Cooking/Burger/BP_BBun` OtherActor))
    (set `self.BBun` _asbp_bbun)
    (if (`SceneComponent.IsVisible` (`self.Plate`))
      ;[1 1 1] Checking if overlapped Component is BBun
      (if (== OtherActor _asbp_bbun)
        (set `self.BBun?` true)
        ;[1 1 1] Checking how the Bun is cooked
        (if (`/Game/Cproef/Blueprints/Cooking/Burger/BP_BBun.IsRaw?` _asbp_bbun)
          (set `self.TotalPoints` (- (`self.TotalPoints`) (`self.PointsRaw`)))
          (`self.AttachToPlate` (`self.BBunLoc`) :!label _label)
          (elif (`/Game/Cproef/Blueprints/Cooking/Burger/BP_BBun.IsCooked?` _asbp_bbun)
            (set `self.TotalPoints` (- (`self.TotalPoints`) (`self.PointsCooked`)))
            (goto _label)
            (elif (`/Game/Cproef/Blueprints/Cooking/Burger/BP_BBun.IsBurned?` _asbp_bbun)
              (set `self.TotalPoints` (- (`self.TotalPoints`) (`self.PointsBurned`)))
              (goto _label))))))))

(event `self.Box2.OnComponentBeginOverlap`
  (params (OverlappedComponent :type "PrimitiveComponent Object Reference") (OtherActor :type "Actor Object Reference") (OtherComp :type "PrimitiveComponent Object Reference") (OtherBodyIndex :type Integer) (bFromSweep :type Boolean) (SweepResult :type "HitResult Structure (by ref)"))
  ;[1 1 1] Putting cheese check
)

(event `self.Box3.OnComponentBeginOverlap`
  (params (OverlappedComponent :type "PrimitiveComponent Object Reference") (OtherActor :type "Actor Object Reference") (OtherComp :type "PrimitiveComponent Object Reference") (OtherBodyIndex :type Integer) (bFromSweep :type Boolean) (SweepResult :type "HitResult Structure (by ref)")))

(event `self.Box4.OnComponentBeginOverlap`
  (params (OverlappedComponent :type "PrimitiveComponent Object Reference") (OtherActor :type "Actor Object Reference") (OtherComp :type "PrimitiveComponent Object Reference") (OtherBodyIndex :type Integer) (bFromSweep :type Boolean) (SweepResult :type "HitResult Structure (by ref)")))

(event `self.Box5.OnComponentBeginOverlap`
  (params (OverlappedComponent :type "PrimitiveComponent Object Reference") (OtherActor :type "Actor Object Reference") (OtherComp :type "PrimitiveComponent Object Reference") (OtherBodyIndex :type Integer) (bFromSweep :type Boolean) (SweepResult :type "HitResult Structure (by ref)")))

(fn `AttachToPlate`
  (params (AttachToParent :type "SceneComponent Object Reference"))
  (`PrimitiveComponent.SetSimulatePhysics` (`self.Plate`) false)
  (`self.K2_AttachToComponent` AttachToParent "None" "SnapToTarget" "SnapToTarget" "KeepRelative"))

(fn `UserConstructionScript`)