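; Plate dispenser for the VR cooking game that spawns a BP_Plate when its button is pressed.
; A Button overlap by a StaticMeshActor or BP_MotionController calls SpawnTopping, which places a scaled plate at SpawnLocation.
; Tick keeps playing a timeline that drives the yaw of RotatePoint.
; Topping spawn, wallet charge and data-table mesh setup remain as disconnected nodes that never run.
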(event `SpawnTopping`
  (bind (_returnvalue_location _returnvalue_rotation) (`KismetMathLibrary.BreakTransform` (`SceneComponent.K2_GetComponentToWorld` (`self.SpawnLocation`))))
  (`|SpawnActorFromClass` "/Game/Cproef/Blueprints/Cooking/BP_Plate.BP_Plate_C" (`KismetMathLibrary.MakeTransform` _returnvalue_location _returnvalue_rotation (2.0 2.0 1.0)) "Undefined" "OverrideRootScale" null null))

(event `self.Button.OnComponentBeginOverlap`
  (params (OverlappedComponent :type "PrimitiveComponent Object Reference") (OtherActor :type "Actor Object Reference") (OtherComp :type "PrimitiveComponent Object Reference") (OtherBodyIndex :type Integer) (bFromSweep :type Boolean) (SweepResult :type "HitResult Structure (by ref)"))
  (bind _returnvalue (`GameplayStatics.GetObjectClass` OtherActor))
  (if (== _returnvalue "/Script/Engine.StaticMeshActor")
    (`self.SpawnTopping` :!label _label)
    (elif (== _returnvalue "/Game/VirtualRealityBP/Blueprints/BP_MotionController.BP_MotionController_C")
      (goto _label))))

(event `self.ReceiveTick`
  (params (DeltaSeconds :type "Float (single-precision)"))
  (bind (_direction _newtrack_0) (`Timeline|Timeline_0`)
    (:`Update`
      (`SceneComponent.K2_SetRelativeRotation` (`self.RotatePoint`) (`KismetMathLibrary.MakeRotator` 0.0 0.0 _newtrack_0) false false))))

(fn `UserConstructionScript`)