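; Cash register actor that slides its mesh and plays a "Kaching" sound when an AI character holds a plate.
; Every tick it gathers all BP_AIChar01 actors and plays a timeline if any has HoldingPlate set.
; The timeline offsets the mesh along world X from the location saved at BeginPlay, and its Finished output leads through a DoOnce Reset to the sound.
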(event `self.ReceiveBeginPlay`
  (set `self.OldLoc` (`SceneComponent.K2_GetComponentLocation` (`self.StaticMeshComponent`))))

(event `self.ReceiveTick`
  (params (DeltaSeconds :type "Float (single-precision)"))
  (bind (_oldloc_x _oldloc_y _oldloc_z) (`KismetMathLibrary.BreakVector` (`self.OldLoc`)))
  (bind _outactors (`GameplayStatics.GetAllActorsOfClass` "/Game/Cproef/test/BP_AIChar01.BP_AIChar01_C"))
  (set `self.AI` _outactors)
  (for _array_element (`self.AI`)
    (if (`/Game/Cproef/test/BP_AIChar01.HoldingPlate?` _array_element)
      (bind (_direction _newtrack_0) (`Timeline|Timeline_0`)
        (:`Update`
          (`SceneComponent.K2_SetWorldLocation` (`self.StaticMeshComponent`) (`KismetMathLibrary.MakeVector` (+ _newtrack_0 _oldloc_x) _oldloc_y _oldloc_z) false false))
        (:`Finished`
          (`/Engine/EditorBlueprintResources/StandardMacros.DoOnce` false :!via `Reset`
            (:`Completed`
              (`GameplayStatics.PlaySoundAtLocation` "/Game/Cproef/Audio/Kaching.Kaching" (`self.OldLoc`) (struct) 1.0 1.0 0.0 null null null))))))))

(fn `UserConstructionScript`)